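; World bag actor that wraps a child-actor BP_Inventory for the player to pick up.
; BeginPlay caches the inventory and tags its owner type, or destroys the actor if the cast fails.
; Overlapping players toggle the prompt widget, and PickUp passes the inventory to the player's InteractBag.
; InitBag, not called here, randomizes loot by removing equipment and backpack items that fail their SpawnRate roll.
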(event `self.ReceiveBeginPlay`
  (bind _asbp_inventory (cast `/Game/GameSrc/Blueprint/ItemContain/BP_Inventory` (`ChildActorComponent.ChildActor` (`self.Inventory`)))
    (:`then`
      (bind _output_get (set `self.InventoryRef` _asbp_inventory))
      (set `/Game/GameSrc/Blueprint/ItemContain/BP_Inventory.InventoryOwner` "NewEnumerator3" _output_get)
      (`SceneComponent.SetVisibility` (`self.Widget`) false false))
    (:`CastFailed`
      (`self.K2_DestroyActor`))))

(event `self.ReceiveActorBeginOverlap`
  (params (OtherActor :type "Actor Object Reference"))
  (if (`KismetSystemLibrary.DoesImplementInterface` OtherActor "/Game/GameSrc/Blueprint/Interface/BPI_IPlayer.BPI_IPlayer_C")
    (`SceneComponent.SetVisibility` (`self.Widget`) true false)))

(event `self.ReceiveActorEndOverlap`
  (params (OtherActor :type "Actor Object Reference"))
  (if (`KismetSystemLibrary.DoesImplementInterface` OtherActor "/Game/GameSrc/Blueprint/Interface/BPI_IPlayer.BPI_IPlayer_C")
    (`SceneComponent.SetVisibility` (`self.Widget`) false false)))

(event `/Game/GameSrc/Blueprint/Interface/BPI_Interact.PickUp`
  (params (InPlayer :type "/Game/GameSrc/Blueprint/Unit/BP_Player Object Reference"))
  (`/Game/GameSrc/Blueprint/Unit/BP_Player.InteractBag` InPlayer (`self.InventoryRef`)))

(fn `GetInventoryRef`
  (returns (InventoryRef :type "/Game/GameSrc/Blueprint/ItemContain/BP_Inventory Object Reference"))
  (return (`self.InventoryRef`)))

(fn `InitBackpackContainer`
  (bind _outbackpack (`/Game/GameSrc/Blueprint/ItemContain/BP_Inventory.GetBackpack` (`self.InventoryRef`)))
  (`/Engine/EditorBlueprintResources/StandardMacros.IsValid` _outbackpack
    (:`Is Valid`
      (for (_array_element _array_index) (`/Game/GameSrc/Blueprint/ItemContain/BP_ItemContainer.ItemSlot` _outbackpack)
        (bind (_instance _quantity _bislock _acceptableenum _acceptableclass) (break `/Game/GameSrc/Blueprint/ItemContain/Structure/ST_FItemContainerSlot` _array_element))
        (bind (_outdata _outisvaliddata) (message `/Game/GameSrc/Blueprint/Interface/BPI_GIHandle.GetItemData` (`GameplayStatics.GetGameInstance`) (`.ItemID_2_8E977A954A28F24960B39DB752D5296B` (break `/Game/GameSrc/Blueprint/ItemContain/Structure/ST_FItemInstance` _instance))))
        (if _outisvaliddata
          (if (>= (`KismetMathLibrary.RandomFloatInRange` 0.0 1.0) (`.SpawnRate_18_37BE0D2641BBC6E30565B19B224615C4` (break `/Game/GameSrc/Blueprint/Item/ST_FItemData` _outdata)))
            (`/Game/GameSrc/Blueprint/Interface/BPI_ItemContain.RemoveItem` (`self.InventoryRef`) _array_index _quantity)))))))

(fn `InitBag`
  (`self.InitBackpackContainer`)
  (`self.InitEquipContainer`))

(fn `InitEquipContainer`
  (bind _outequip (`/Game/GameSrc/Blueprint/ItemContain/BP_Inventory.GetEquip` (`self.InventoryRef`)))
  (`/Engine/EditorBlueprintResources/StandardMacros.IsValid` _outequip
    (:`Is Valid`
      (for (_array_element _array_index) (`/Game/GameSrc/Blueprint/ItemContain/BP_ItemContainer.ItemSlot` _outequip)
        (bind (_instance _quantity _bislock _acceptableenum _acceptableclass) (break `/Game/GameSrc/Blueprint/ItemContain/Structure/ST_FItemContainerSlot` _array_element))
        (bind (_outdata _outisvaliddata) (message `/Game/GameSrc/Blueprint/Interface/BPI_GIHandle.GetItemData` (`GameplayStatics.GetGameInstance`) (`.ItemID_2_8E977A954A28F24960B39DB752D5296B` (break `/Game/GameSrc/Blueprint/ItemContain/Structure/ST_FItemInstance` _instance))))
        (if _outisvaliddata
          (if (>= (`KismetMathLibrary.RandomFloatInRange` 0.0 1.0) (`.SpawnRate_18_37BE0D2641BBC6E30565B19B224615C4` (break `/Game/GameSrc/Blueprint/Item/ST_FItemData` _outdata)))
            (`/Game/GameSrc/Blueprint/Interface/BPI_ItemContain.RemoveItem` _outequip _array_index _quantity)))))))

(fn `UserConstructionScript`)