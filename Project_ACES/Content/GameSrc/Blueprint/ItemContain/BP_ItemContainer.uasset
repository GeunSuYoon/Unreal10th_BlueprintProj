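; BP_ItemContainer is an inventory container that holds items in a fixed array of slots, sized on BeginPlay and resizable.
; Adding stacks onto matching items up to MaxStack from GameInstance data, spills overflow into other slots and accumulates weight; targeted adds also check each slot's accepted class.
; MoveItem transfers between containers with re-add on failure, while DropItem spawns BP_PickupItem.
; Change dispatchers announce updates; removal leaves weight untouched, and SwapItemContainer and RemoveItemSlot are stubs.
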(event `self.ReceiveBeginPlay`
  (for _ (range (`self.MaxSlotSize`))
    (`KismetArrayLibrary.Array_Add` (`self.ItemSlot`) (make `/Game/GameSrc/Blueprint/ItemContain/Structure/ST_FItemContainerSlot` (struct :`ItemType` "NewEnumerator6" :`WeaponState` (struct) :`UnitPartsState` (struct :`PartsType` "NewEnumerator5")) 0 false "NewEnumerator9" "/Game/GameSrc/Blueprint/Item/BP_Item.BP_Item_C"))))

(fn `AddItem`
  (params (InData :type "/Game/GameSrc/Blueprint/ItemContain/Structure/ST_FItemInstance Structure") (InCount :type Integer))
  (returns (bOutIsSuccess :type Boolean))
  ;[0.15 0.15 0.15 0.5 15] 동일 아이템 있는지 찾기
  (bind _outidx (`self.FindItemIdx` InData))
  ;[0.15 0.15 0.15 0.5 15] T: 있다 F: 없다
  (if (!= _outidx -1)
    ;[0.15 0.15 0.15 0.5 15] 있으면 일단 다 넣는다
    (bind _outquantity (`self.UpdateSlotCount` InData _outidx InCount))
    ;[0.15 0.15 0.15 0.5 15] 넣고 남은 양 유무 확인
    (if (== _outquantity 0)
      ;[0.15 0.15 0.15 0.5 15] 남은거 없다
      (`self.OnInventoryChange` _outidx)
      (else
        ;[0.15 0.15 0.15 0.5 15] 남은거 있음 빈자리에 넣기
        (`self.OnInventoryChange` _outidx)
        (bind _outindex (`self.FindEmptySlot` 0))
        (bind _boutissuccess (`/Game/GameSrc/Blueprint/Interface/BPI_ItemContain.AddItemSlot` InData _outindex _outquantity))
        (return _boutissuccess)))
    (else
      ;[0.15 0.15 0.15 0.5 15] 빈 슬롯 찾기
      (bind _outindex_2 (`self.FindEmptySlot` (+ _outidx 1)))
      ;[0.15 0.15 0.15 0.5 15] T: 빈 슬롯 있다 F: 빈 슬롯 없다
      (if (!= _outindex_2 -1)
        ;[0.15 0.15 0.15 0.5 15] 빈 슬롯에 넣고 슬롯 사이즈 업데이트
        (`self.UpdateSlot` InData _outindex_2 InCount)
        (`/Engine/EditorBlueprintResources/StandardMacros.IncrementInt` (`self.CurrentSlotSize`)
          (:`  `
            (`self.OnInventoryChange` _outindex_2)))
        (else
          (return false)))))
  (`self.OnMaxSlotSizeChange`)
  (return true))

(fn `AddItemSlot`
  (params (InData :type "/Game/GameSrc/Blueprint/ItemContain/Structure/ST_FItemInstance Structure") (InSlotIdx :type Integer) (InCount :type Integer))
  (returns (bOutIsSuccess :type Boolean))
  ;[0.15 0.15 0.15 0.5 15] 제대로된 인덱스가 들어왔나
  (if (`KismetArrayLibrary.Array_IsValidIndex` (`self.ItemSlot`) InSlotIdx)
    ;[0.15 0.15 0.15 0.5 15] 슬롯에 들어갈 수 있는 아이템이 들어왔나
    (bind _bisaccept (`self.bIsAcceptItem` InData InSlotIdx))
    (if _bisaccept
      ;[0.15 0.15 0.15 0.5 15] 슬롯이 비어있나
      (bind _outisempty (`self.bIsEmptySlot` InSlotIdx))
      (if _outisempty
        (`self.UpdateSlot` InData InSlotIdx InCount)
        (`/Engine/EditorBlueprintResources/StandardMacros.IncrementInt` (`self.CurrentSlotSize`)
          (:`  `
            _))
        (else
          ;[0.15 0.15 0.15 0.5 15] 슬롯에 들어있는 아이템과 같은 아이템이냐
          (bind _outissame (`self.bIsSameItemSlot` InData InSlotIdx))
          (if _outissame
            ;[0.15 0.15 0.15 0.5 15] 아이템 넣고 남냐
            (bind _outquantity (`self.UpdateSlotCount` InData InSlotIdx InCount))
            (if (== _outquantity 0)
              _
              (else
                (`self.OnInventoryChange` InSlotIdx)
                (`self.OnMaxSlotSizeChange`)
                (bind _boutissuccess (`/Game/GameSrc/Blueprint/Interface/BPI_ItemContain.AddItem` InData _outquantity))
                (return _boutissuccess)))
            (else
              (bind _boutissuccess_2 (`/Game/GameSrc/Blueprint/Interface/BPI_ItemContain.AddItem` (struct) InCount))
              (return _boutissuccess_2)))))
      (`self.OnInventoryChange` InSlotIdx)
      (`self.OnMaxSlotSizeChange`)
      (return true)
      (else
        _)))
  (return false))

(fn `AddWeight`
  (params (InWeight :type "Float (double-precision)"))
  (set `self.CurrentWeight` (+ InWeight (`self.CurrentWeight`))))

(fn `bIsAcceptItem`
  (params (InData :type "/Game/GameSrc/Blueprint/ItemContain/Structure/ST_FItemInstance Structure") (InIdx :type Integer))
  (returns (bIsAccept :type Boolean))
  (bind (_outdata _outisvaliddata) (message `/Game/GameSrc/Blueprint/Interface/BPI_DataTableHandle.GetItemData` (`GameplayStatics.GetGameInstance`) (`.ItemID_2_8E977A954A28F24960B39DB752D5296B` (break `/Game/GameSrc/Blueprint/ItemContain/Structure/ST_FItemInstance` InData))))
  (if _outisvaliddata
    (return (`KismetMathLibrary.ClassIsChildOf` (`.BPClass_15_0FF1DB7244244BF787F18CAE07DBDB55` (break `/Game/GameSrc/Blueprint/Item/ST_FItemData` _outdata)) (`.AcceptableClass_29_FD10037D40575C4380597FA5874380A5` (break `/Game/GameSrc/Blueprint/ItemContain/Structure/ST_FItemContainerSlot` (`|GetArrayItem` (`self.ItemSlot`) InIdx)))))
    (else
      (return false))))

(fn `bIsEmptySlot`
  (params (InIdx :type Integer))
  (returns (OutIsEmpty :type Boolean))
  (return (== (`.Quantity_10_B3ECC0C94CC79C082E5E27B4736CC1B3` (break `/Game/GameSrc/Blueprint/ItemContain/Structure/ST_FItemContainerSlot` (`|GetArrayItem` (`self.ItemSlot`) InIdx))) 0)))

(fn `bIsSameItemSlot`
  (params (InData :type "/Game/GameSrc/Blueprint/ItemContain/Structure/ST_FItemInstance Structure") (InIdx :type Integer))
  (returns (OutIsSame :type Boolean))
  (return (== (`.ItemID_2_8E977A954A28F24960B39DB752D5296B` (break `/Game/GameSrc/Blueprint/ItemContain/Structure/ST_FItemInstance` InData)) (`.ItemID_2_8E977A954A28F24960B39DB752D5296B` (break `/Game/GameSrc/Blueprint/ItemContain/Structure/ST_FItemInstance` (`.Instance_25_BEE9DDFB4DA2EACA0AED239E490E0271` (break `/Game/GameSrc/Blueprint/ItemContain/Structure/ST_FItemContainerSlot` (`|GetArrayItem` (`self.ItemSlot`) InIdx))))))))

(fn `ChunkItem`
  (params (InIdx :type Integer) (InCount :type Integer) (InTransform :type "Transform Structure"))
  (locals (TargetInstance :type "/Game/GameSrc/Blueprint/ItemContain/Structure/ST_FItemInstance Structure"))
  (set `local.TargetInstance` (`.Instance_25_BEE9DDFB4DA2EACA0AED239E490E0271` (break `/Game/GameSrc/Blueprint/ItemContain/Structure/ST_FItemContainerSlot` (`|GetArrayItem` (`self.ItemSlot`) InIdx))))
  (bind _bissuccess (`/Game/GameSrc/Blueprint/Interface/BPI_ItemContain.RemoveItem` InIdx InCount))
  (if _bissuccess
    (`|SpawnActorFromClass` "/Game/GameSrc/Blueprint/Item/BP_PickupItem.BP_PickupItem_C" InTransform "Undefined" "MultiplyWithRoot" null null)))

(fn `DropItem`
  (params (InIdx :type Integer) (InCount :type Integer) (InTransform :type "Transform Structure"))
  (returns (OutIsVal :type Boolean))
  (locals (TargetInstance :type "/Game/GameSrc/Blueprint/ItemContain/Structure/ST_FItemInstance Structure"))
  (bind _output_get (set `local.TargetInstance` (`.Instance_25_BEE9DDFB4DA2EACA0AED239E490E0271` (break `/Game/GameSrc/Blueprint/ItemContain/Structure/ST_FItemContainerSlot` (`|GetArrayItem` (`self.ItemSlot`) InIdx)))))
  (bind _bissuccess (`/Game/GameSrc/Blueprint/Interface/BPI_ItemContain.RemoveItem` InIdx InCount))
  (if _bissuccess
    (`|SpawnActorFromClass` "/Game/GameSrc/Blueprint/Item/BP_PickupItem.BP_PickupItem_C" InTransform "Undefined" "MultiplyWithRoot" null null _output_get InCount)
    (return true)
    (else
      (return false))))

(fn `FindEmptySlot`
  (params (InStartIdx :type Integer))
  (returns (OutIndex :type Integer))
  (bind _itemslot (`self.ItemSlot`))
  (if (`KismetArrayLibrary.Array_IsEmpty` _itemslot)
    (return 0)
    (else
      (for _index (range InStartIdx (`self.MaxSlotSize`))
        (if (== 0 (`.Quantity_10_B3ECC0C94CC79C082E5E27B4736CC1B3` (break `/Game/GameSrc/Blueprint/ItemContain/Structure/ST_FItemContainerSlot` (`|GetArrayItem` _itemslot _index))))
          (return _index)))
      (return -1))))

(fn `FindItemIdx`
  (params (InData :type "/Game/GameSrc/Blueprint/ItemContain/Structure/ST_FItemInstance Structure"))
  (returns (OutIdx :type Integer))
  (for (_array_element _array_index) (`self.ItemSlot`)
    (if (== (`.ItemID_2_8E977A954A28F24960B39DB752D5296B` (break `/Game/GameSrc/Blueprint/ItemContain/Structure/ST_FItemInstance` InData)) (`.ItemID_2_8E977A954A28F24960B39DB752D5296B` (break `/Game/GameSrc/Blueprint/ItemContain/Structure/ST_FItemInstance` (`.Instance_25_BEE9DDFB4DA2EACA0AED239E490E0271` (break `/Game/GameSrc/Blueprint/ItemContain/Structure/ST_FItemContainerSlot` _array_element)))))
      (return _array_index)))
  (return -1))

(fn `GetItem`
  (params (InIdx :type Integer))
  (returns (OutData :type "/Game/GameSrc/Blueprint/ItemContain/Structure/ST_FItemInstance Structure"))
  (bind _itemslot (`self.ItemSlot`))
  (if (`KismetArrayLibrary.Array_IsValidIndex` _itemslot InIdx)
    (return (`.Instance_25_BEE9DDFB4DA2EACA0AED239E490E0271` (break `/Game/GameSrc/Blueprint/ItemContain/Structure/ST_FItemContainerSlot` (`|GetArrayItem` _itemslot InIdx))))
    (else
      (return))))

(fn `GetItemWeight`
  (params (InData :type "/Game/GameSrc/Blueprint/ItemContain/Structure/ST_FItemInstance Structure") (InCount :type Integer))
  (returns (OutWeight :type "Float (double-precision)"))
  (bind (_outweight _outisvaliddata) (message `/Game/GameSrc/Blueprint/Interface/BPI_DataTableHandle.GetItemWeight` (`GameplayStatics.GetGameInstance`) (`.ItemID_2_8E977A954A28F24960B39DB752D5296B` (break `/Game/GameSrc/Blueprint/ItemContain/Structure/ST_FItemInstance` InData))))
  (if _outisvaliddata
    (return (* _outweight InCount))
    (else
      (return 0.0))))

(fn `IsEmptySlot`
  (params (InIdx :type Integer))
  (returns (OutIsEmpty :type Boolean))
  (return (!= (`.Quantity_10_B3ECC0C94CC79C082E5E27B4736CC1B3` (break `/Game/GameSrc/Blueprint/ItemContain/Structure/ST_FItemContainerSlot` (`|GetArrayItem` (`self.ItemSlot`) InIdx))) 0)))

(fn `MoveItem`
  (params (SourceContainer :type "/Game/GameSrc/Blueprint/Interface/BPI_ItemContain Interface") (TargetContainer :type "/Game/GameSrc/Blueprint/Interface/BPI_ItemContain Interface") (SourceIdx :type Integer) (TargetIdx :type Integer) (InData :type "/Game/GameSrc/Blueprint/ItemContain/Structure/ST_FItemInstance Structure") (MoveCount :type Integer))
  (returns (bIsMoveSuccess :type Boolean))
  (bind _bisaccept (`/Game/GameSrc/Blueprint/Interface/BPI_ItemContain.bIsAcceptItem` TargetContainer InData 0))
  (if _bisaccept
    (bind _bissuccess (`/Game/GameSrc/Blueprint/Interface/BPI_ItemContain.RemoveItem` SourceContainer SourceIdx MoveCount))
    (bind _outdata (`/Game/GameSrc/Blueprint/Interface/BPI_ItemContain.GetItem` SourceContainer SourceIdx))
    (if _bissuccess
      (bind _boutissuccess (`/Game/GameSrc/Blueprint/Interface/BPI_ItemContain.AddItemSlot` TargetContainer _outdata TargetIdx MoveCount))
      (if _boutissuccess
        (return true)
        (else
          (`/Game/GameSrc/Blueprint/Interface/BPI_ItemContain.AddItemSlot` SourceContainer _outdata SourceIdx MoveCount)))))
  (return false))

(fn `RemoveItem`
  (params (InIdx :type Integer) (InCount :type Integer))
  (returns (bIsSuccess :type Boolean))
  (bind _itemslot (`self.ItemSlot`))
  (bind (_instance _quantity _bislock) (break `/Game/GameSrc/Blueprint/ItemContain/Structure/ST_FItemContainerSlot` (`|GetArrayItem` _itemslot InIdx)))
  (if (`KismetArrayLibrary.Array_IsValidIndex` _itemslot InIdx)
    (if (< _quantity InCount)
      (`KismetArrayLibrary.Array_Remove` _itemslot InIdx)
      (else
        (`KismetArrayLibrary.Array_Set` _itemslot InIdx (make `/Game/GameSrc/Blueprint/ItemContain/Structure/ST_FItemContainerSlot` _instance (- _quantity InCount) _bislock "NewEnumerator9" null))))
    (`/Engine/EditorBlueprintResources/StandardMacros.DecrementInt` (`self.CurrentSlotSize`)
      (:`  `
        (`self.OnInventoryChange` InIdx)
        (`self.OnMaxSlotSizeChange`)
        (return true)))
    (else
      (return false))))

(fn `RemoveItemSlot`
  (params (InData :type "/Game/GameSrc/Blueprint/ItemContain/Structure/ST_FItemInstance Structure") (InSlotIdx :type Integer) (InCount :type Integer))
  (returns (bIsSuccess :type Boolean))
  (return false))

(fn `SetMaxSlotSize`
  (params (InSize :type Integer))
  (bind _itemslot (`self.ItemSlot`))
  (if (not (> InSize (`self.MaxSlotSize`)))
    (for _array_element _itemslot
      (if (!= (`.Quantity_10_B3ECC0C94CC79C082E5E27B4736CC1B3` (break `/Game/GameSrc/Blueprint/ItemContain/Structure/ST_FItemContainerSlot` _array_element)) 0)
        (return))))
  (bind _output_get (set `self.MaxSlotSize` InSize))
  (`KismetArrayLibrary.Array_Resize` _itemslot _output_get)
  (`self.OnMaxSlotSizeChange`))

(fn `SwapItem`
  (params (InIdx1 :type Integer) (InIdx2 :type Integer))
  (returns (bIsSwapSuccess :type Boolean))
  (locals (TempItem :type "/Game/GameSrc/Blueprint/ItemContain/Structure/ST_FItemContainerSlot Structure"))
  (bind _itemslot (`self.ItemSlot`))
  (bind _output_get (set `local.TempItem` (`|GetArrayItem` _itemslot InIdx1)))
  (`KismetArrayLibrary.Array_Set` _itemslot InIdx1 (`|GetArrayItem` _itemslot InIdx2))
  (`KismetArrayLibrary.Array_Set` _itemslot InIdx2 _output_get)
  (return true))

(fn `SwapItemContainer`)

(fn `UpdateSlot`
  (params (InData :type "/Game/GameSrc/Blueprint/ItemContain/Structure/ST_FItemInstance Structure") (InIdx :type Integer) (InQuantity :type Integer))
  (bind _itemslot (`self.ItemSlot`))
  (bind (_instance _quantity _bislock _acceptableenum _acceptableclass) (break `/Game/GameSrc/Blueprint/ItemContain/Structure/ST_FItemContainerSlot` (`|GetArrayItem` _itemslot InIdx)))
  (bind (_outdata _outisvaliddata) (message `/Game/GameSrc/Blueprint/Interface/BPI_DataTableHandle.GetItemData` (`GameplayStatics.GetGameInstance`) (`.ItemID_2_8E977A954A28F24960B39DB752D5296B` (break `/Game/GameSrc/Blueprint/ItemContain/Structure/ST_FItemInstance` InData))))
  (if _outisvaliddata
    (bind _outweight (`/Game/GameSrc/Blueprint/Interface/BPI_ItemContain.GetItemWeight` InData InQuantity))
    (`self.AddWeight` _outweight)
    (`KismetArrayLibrary.Array_Set` _itemslot InIdx (make `/Game/GameSrc/Blueprint/ItemContain/Structure/ST_FItemContainerSlot` InData InQuantity _bislock _acceptableenum _acceptableclass))))

(fn `UpdateSlotCount`
  (params (InData :type "/Game/GameSrc/Blueprint/ItemContain/Structure/ST_FItemInstance Structure") (InIdx :type Integer) (InQuantity :type Integer))
  (returns (OutQuantity :type Integer))
  (bind _itemslot (`self.ItemSlot`))
  (bind (_instance _quantity _bislock _acceptableenum _acceptableclass) (break `/Game/GameSrc/Blueprint/ItemContain/Structure/ST_FItemContainerSlot` (`|GetArrayItem` _itemslot InIdx)))
  (bind _returnvalue (+ _quantity InQuantity))
  (bind (_outdata _outisvaliddata) (message `/Game/GameSrc/Blueprint/Interface/BPI_DataTableHandle.GetItemData` (`GameplayStatics.GetGameInstance`) (`.ItemID_2_8E977A954A28F24960B39DB752D5296B` (break `/Game/GameSrc/Blueprint/ItemContain/Structure/ST_FItemInstance` _instance))))
  (if _outisvaliddata
    (bind (_id _name _rarity _itemtype _buyprice _saleprice _weight _bpclass _spawnrate _mesh _image _maxstack) (break `/Game/GameSrc/Blueprint/Item/ST_FItemData` _outdata))
    ;[0.15 0.15 0.15 0.5 15] 추가한 개수가 아이템 최대 스택보다 작냐
    (if (<= _returnvalue _maxstack)
      ;[0.15 0.15 0.15 0.5 15] 작으면 넣고 남은 개수 0개 리턴
      (bind _outweight (`self.GetItemWeight` _instance InQuantity))
      (`self.AddWeight` _outweight)
      (`KismetArrayLibrary.Array_Set` _itemslot InIdx (make `/Game/GameSrc/Blueprint/ItemContain/Structure/ST_FItemContainerSlot` _instance _returnvalue _bislock _acceptableenum _acceptableclass))
      (return 0)
      (else
        ;[0.15 0.15 0.15 0.5 15] 크면 최대치 넣고 남은 개수 리턴
        (bind _outweight_2 (`self.GetItemWeight` _instance (- _maxstack _quantity)))
        (`self.AddWeight` _outweight_2)
        (`KismetArrayLibrary.Array_Set` _itemslot InIdx (make `/Game/GameSrc/Blueprint/ItemContain/Structure/ST_FItemContainerSlot` _instance _maxstack _bislock _acceptableenum _acceptableclass))
        (return (- _returnvalue _maxstack))))
    (else
      (return 0))))