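; BP_Inventory is an inventory facade that owns a backpack container and an equipment container, using its parent actor's transform for item actions.
; InitInventory initializes both containers, seeding equipment slots with hard-coded test items through TestEquip before InitEquip.
; OnContextClick routes slot actions by owner, passing the opposite container along.
; AddItem forwards to the backpack, while the other item operations are stubs returning default values.
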(event `self.ReceiveBeginPlay`)

(fn `AddItem`
  (params (InData :type "/Game/GameSrc/Blueprint/ItemContain/Structure/ST_FItemInstance Structure") (InCount :type Integer))
  (returns (bOutIsSuccess :type Boolean))
  (bind _boutissuccess (`/Game/GameSrc/Blueprint/Interface/BPI_ItemContain.AddItem` (`self.BP_BackpackContainer`) InData InCount))
  (return _boutissuccess))

(fn `AddItemSlot`
  (params (InData :type "/Game/GameSrc/Blueprint/ItemContain/Structure/ST_FItemInstance Structure") (InSlotIdx :type Integer) (InCount :type Integer))
  (returns (bOutIsSuccess :type Boolean))
  (return false))

(fn `bIsAcceptItem`
  (params (InData :type "/Game/GameSrc/Blueprint/ItemContain/Structure/ST_FItemInstance Structure") (InIdx :type Integer))
  (returns (bIsAccept :type Boolean))
  (return false))

(fn `GetBackpack`
  (returns (OutBackpack :type "/Game/GameSrc/Blueprint/ItemContain/BP_BackpackContainer Object Reference"))
  (return (`self.BP_BackpackContainer`)))

(fn `GetEquip`
  (returns (OutEquip :type "/Game/GameSrc/Blueprint/ItemContain/BP_EquipContainer Object Reference"))
  (return (`self.BP_EquipContainer`)))

(fn `GetItem`
  (params (InIdx :type Integer))
  (returns (OutData :type "/Game/GameSrc/Blueprint/ItemContain/Structure/ST_FItemInstance Structure"))
  (return))

(fn `GetItemWeight`
  (params (InData :type "/Game/GameSrc/Blueprint/ItemContain/Structure/ST_FItemInstance Structure") (InCount :type Integer))
  (returns (OutWeight :type "Float (double-precision)"))
  (return 0.0))

(fn `InitInventory`
  (`/Game/GameSrc/Blueprint/ItemContain/BP_BackpackContainer.InitBackpack` (`self.BP_BackpackContainer`))
  (`self.TestEquip`)
  (`/Game/GameSrc/Blueprint/ItemContain/BP_EquipContainer.InitEquip` (`self.BP_EquipContainer`)))

(fn `IsEmptySlot`
  (params (InIdx :type Integer))
  (returns (OutIsEmpty :type Boolean))
  (return false))

(fn `MoveItem`
  (params (SourceContainer :type "/Game/GameSrc/Blueprint/Interface/BPI_ItemContain Interface") (TargetContainer :type "/Game/GameSrc/Blueprint/Interface/BPI_ItemContain Interface") (SourceIdx :type Integer) (TargetIdx :type Integer) (InData :type "/Game/GameSrc/Blueprint/ItemContain/Structure/ST_FItemInstance Structure") (MoveCount :type Integer))
  (returns (bIsMoveSuccess :type Boolean))
  (return false))

(fn `OnContextClick`
  (params (InSlotOwn :type "/Game/GameSrc/Blueprint/Widget/HUD/Inventory/EOwnInventoryType Enum" :default "NewEnumerator0") (InSlotIdx :type Integer) (InContextAction :type "/Game/GameSrc/Blueprint/Widget/HUD/Inventory/ButtenContext/EContextActionType Enum" :default "NewEnumerator0"))
  (bind _bp_backpackcontainer (`self.BP_BackpackContainer`))
  (bind _bp_equipcontainer (`self.BP_EquipContainer`))
  (bind _returnvalue (`self.GetTransform` (`self.GetParentActor`)))
  (switch `/Game/GameSrc/Blueprint/Widget/HUD/Inventory/EOwnInventoryType` InSlotOwn
    (:`NewEnumerator0`
      (`/Game/GameSrc/Blueprint/ItemContain/BP_EquipContainer.OnContextClick` _bp_equipcontainer InSlotIdx InContextAction _bp_backpackcontainer _returnvalue))
    (:`NewEnumerator1`
      (`/Game/GameSrc/Blueprint/ItemContain/BP_BackpackContainer.OnContextClick` _bp_backpackcontainer InSlotIdx InContextAction _bp_equipcontainer _returnvalue))))

(fn `RemoveItem`
  (params (InIdx :type Integer) (InCount :type Integer))
  (returns (bIsSuccess :type Boolean))
  (return false))

(fn `RemoveItemSlot`
  (params (InData :type "/Game/GameSrc/Blueprint/ItemContain/Structure/ST_FItemInstance Structure") (InSlotIdx :type Integer) (InCount :type Integer))
  (returns (bIsSuccess :type Boolean))
  (return false))

(fn `TestEquip`
  (bind _bp_equipcontainer (`self.BP_EquipContainer`))
  (bind _st_fiteminstance (make `/Game/GameSrc/Blueprint/ItemContain/Structure/ST_FItemInstance` "21001" "NewEnumerator6" (make `/Game/GameSrc/Blueprint/ItemContain/Structure/ST_FWeaponState` 100.0 0 null null null)))
  (`/Game/GameSrc/Blueprint/ItemContain/BP_ItemContainer.UpdateSlot` _bp_equipcontainer (make `/Game/GameSrc/Blueprint/ItemContain/Structure/ST_FItemInstance` "11001" "NewEnumerator6" (make `/Game/GameSrc/Blueprint/ItemContain/Structure/ST_FWeaponState` 100.0 0 null null null)) 0 1)
  (`/Game/GameSrc/Blueprint/ItemContain/BP_ItemContainer.UpdateSlot` _bp_equipcontainer (make `/Game/GameSrc/Blueprint/ItemContain/Structure/ST_FItemInstance` "13001" "NewEnumerator6" (make `/Game/GameSrc/Blueprint/ItemContain/Structure/ST_FWeaponState` 100.0 0 null null null)) 2 1)
  (`/Game/GameSrc/Blueprint/ItemContain/BP_ItemContainer.UpdateSlot` _bp_equipcontainer _st_fiteminstance 4 1)
  (`/Game/GameSrc/Blueprint/ItemContain/BP_ItemContainer.UpdateSlot` _bp_equipcontainer _st_fiteminstance 5 1))

(fn `UserConstructionScript`)