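; Equipment variant of an item container, where items are placed into specific typed slots.
; AddItemSlot runs the parent logic, then calls CallOnEquipChange with the item data and that slot's accepted type, regardless of the parent's result.
; Generic AddItem always returns false, so it never auto-places items.
; Weight, removal, acceptance and lookup defer to the parent, so removal raises no equip-change call here.
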(fn `AddItem`
  (params (InData :type "/Game/GameSrc/Blueprint/Item/ST_FItemData Structure") (InCount :type Integer))
  (returns (bOutIsSuccess :type Boolean))
  (return false))

(fn `AddItemSlot`
  (params (InData :type "/Game/GameSrc/Blueprint/Item/ST_FItemData Structure") (InSlotIdx :type Integer) (InCount :type Integer))
  (returns (bOutIsSuccess :type Boolean))
  (bind _boutissuccess (`parent.AddItemSlot` InData InSlotIdx InCount))
  (`self.OnEquipChange` InData (`.AcceptableEnum_21_072452B74F3EAB16ED5149A8352430D1` (break `/Game/GameSrc/Blueprint/ItemContain/ST_FItemContainerSlot` (`|GetArrayItem` (`self.ItemSlot`) InSlotIdx))))
  (return _boutissuccess))

(fn `bIsAcceptItem`
  (params (InData :type "/Game/GameSrc/Blueprint/Item/ST_FItemData Structure") (InIdx :type Integer))
  (returns (bIsAccept :type Boolean))
  (bind _bisaccept (`parent.bIsAcceptItem` InData InIdx))
  (return _bisaccept))

(fn `GetItem`
  (params (InIdx :type Integer))
  (returns (OutData :type "/Game/GameSrc/Blueprint/Item/ST_FItemData Structure"))
  (bind _outdata (`parent.GetItem` InIdx))
  (return _outdata))

(fn `GetItemWeight`
  (params (InData :type "/Game/GameSrc/Blueprint/Item/ST_FItemData Structure") (InCount :type Integer))
  (returns (OutWeight :type "Float (double-precision)"))
  (bind _outweight (`parent.GetItemWeight` InData InCount))
  (return _outweight))

(fn `RemoveItem`
  (params (InIdx :type Integer) (InCount :type Integer))
  (returns (bIsSuccess :type Boolean))
  (bind _bissuccess (`parent.RemoveItem` InIdx InCount))
  (return _bissuccess))