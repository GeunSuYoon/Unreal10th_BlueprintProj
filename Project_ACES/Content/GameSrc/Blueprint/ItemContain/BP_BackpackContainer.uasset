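; Backpack item container that extends a parent container with slot context actions for dropping and equipping items.
; Most item operations defer to the parent; removal also subtracts from CurrentWeight, while the weight increment on adding is disconnected.
; EquipItem looks up item data through the GameInstance, then moves unit parts to their type's slot or weapons to the first free of two weapon slots.
; InitBackpack broadcasts every slot and the slot capacity to listeners.
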(event `self.ReceiveBeginPlay`
  (`parent.ReceiveBeginPlay`))

(fn `AddItem`
  (params (InData :type "/Game/GameSrc/Blueprint/ItemContain/Structure/ST_FItemInstance Structure") (InCount :type Integer))
  (returns (bOutIsSuccess :type Boolean))
  (bind _boutissuccess (`parent.AddItem` InData InCount))
  (if _boutissuccess
    (`KismetSystemLibrary.PrintString` "Hello")
    (return true)
    (else
      (return false))))

(fn `AddItemSlot`
  (params (InData :type "/Game/GameSrc/Blueprint/ItemContain/Structure/ST_FItemInstance Structure") (InSlotIdx :type Integer) (InCount :type Integer))
  (returns (bOutIsSuccess :type Boolean))
  (bind _boutissuccess (`parent.AddItemSlot` InData InSlotIdx InCount))
  (if _boutissuccess
    (return true)
    (else
      (return false))))

(fn `bIsAcceptItem`
  (params (InData :type "/Game/GameSrc/Blueprint/ItemContain/Structure/ST_FItemInstance Structure") (InIdx :type Integer))
  (returns (bIsAccept :type Boolean))
  (bind _bisaccept (`parent.bIsAcceptItem` InData InIdx))
  (return _bisaccept))

(fn `DropItem`
  (params (InIdx :type Integer) (InCount :type Integer) (InTransform :type "Transform Structure"))
  (returns (OutIsVal :type Boolean))
  (bind _outisval (`parent.DropItem` InIdx InCount InTransform))
  (return _outisval))

(fn `EquipItem`
  (params (InIdx :type Integer) (InContainer :type "/Game/GameSrc/Blueprint/Interface/BPI_ItemContain Interface"))
  (returns (OutIsEquip :type Boolean))
  (bind _returnvalue (`GameplayStatics.GetGameInstance`))
  (bind (_instance _quantity) (break `/Game/GameSrc/Blueprint/ItemContain/Structure/ST_FItemContainerSlot` (`|GetArrayItem` (`self.ItemSlot`) InIdx)))
  (bind (_outdata _outisvaliddata) (message `/Game/GameSrc/Blueprint/Interface/BPI_GIHandle.GetItemData` _returnvalue (`.ItemID_2_8E977A954A28F24960B39DB752D5296B` (break `/Game/GameSrc/Blueprint/ItemContain/Structure/ST_FItemInstance` _instance))))
  (if _outisvaliddata
    (bind (_id _name _rarity _itemtype) (break `/Game/GameSrc/Blueprint/Item/ST_FItemData` _outdata))
    (switch `/Game/GameSrc/Blueprint/Item/EItemType` _itemtype
      (:`NewEnumerator0`
        (bind (_outdata_2 _outisvaliddata_2) (message `/Game/GameSrc/Blueprint/Interface/BPI_GIHandle.GetUnitPartsData` _returnvalue _id))
        (if _outisvaliddata_2
          (bind _returnvalue_2 (- (`KismetMathLibrary.Conv_ByteToInt` (`.PartsType_9_543EAEA0432F59176BB0AEA58949A9F3` (break `/Game/GameSrc/Blueprint/Item/UnitParts/ST_UnitPartsData` _outdata_2))) 1))
          (bind _outisempty (`/Game/GameSrc/Blueprint/Interface/BPI_ItemContain.IsEmptySlot` InContainer _returnvalue_2))
          (if _outisempty
            (bind _bismovesuccess (`/Game/GameSrc/Blueprint/Interface/BPI_ItemContain.MoveItem` self InContainer InIdx _returnvalue_2 _instance _quantity))
            (return _bismovesuccess))
          (else
            (return false))))
      (:`NewEnumerator1`
        (bind _outisempty_2 (`/Game/GameSrc/Blueprint/Interface/BPI_ItemContain.IsEmptySlot` InContainer 4))
        (if _outisempty_2
          (bind _bismovesuccess_2 (`/Game/GameSrc/Blueprint/Interface/BPI_ItemContain.MoveItem` self InContainer InIdx 4 _instance _quantity))
          (if _bismovesuccess_2
            (`self.OnEquipSuccess`)
            (return true)
            (else
              _))
          (else
            (bind _outisempty_3 (`/Game/GameSrc/Blueprint/Interface/BPI_ItemContain.IsEmptySlot` InContainer 5))
            (if _outisempty_3
              (bind _bismovesuccess_3 (`/Game/GameSrc/Blueprint/Interface/BPI_ItemContain.MoveItem` self InContainer InIdx 5 _instance _quantity))
              (if _bismovesuccess_3
                (`self.OnEquipSuccess`)
                (return true)
                (else
                  _))
              (else
                (return false)))))
        (return false)))
    (else
      (return false))))

(fn `EquipItemTmp`
  (params (InIdx :type Integer) (InEquipContainer :type "/Game/GameSrc/Blueprint/Interface/BPI_ItemContain Interface")))

(fn `GetItem`
  (params (InIdx :type Integer))
  (returns (OutData :type "/Game/GameSrc/Blueprint/ItemContain/Structure/ST_FItemInstance Structure"))
  (bind _outdata (`parent.GetItem` InIdx))
  (return _outdata))

(fn `GetItemWeight`
  (params (InData :type "/Game/GameSrc/Blueprint/ItemContain/Structure/ST_FItemInstance Structure") (InCount :type Integer))
  (returns (OutWeight :type "Float (double-precision)"))
  (bind _outweight (`parent.GetItemWeight` InData InCount))
  (return _outweight))

(fn `InitBackpack`
  (for (_ _array_index) (`self.ItemSlot`)
    (`self.OnInventoryChange` _array_index))
  (`self.OnMaxSlotSizeChange`))

(fn `MoveItem`
  (params (SourceContainer :type "/Game/GameSrc/Blueprint/Interface/BPI_ItemContain Interface") (TargetContainer :type "/Game/GameSrc/Blueprint/Interface/BPI_ItemContain Interface") (SourceIdx :type Integer) (TargetIdx :type Integer) (InData :type "/Game/GameSrc/Blueprint/ItemContain/Structure/ST_FItemInstance Structure") (MoveCount :type Integer))
  (returns (bIsMoveSuccess :type Boolean))
  (bind _bismovesuccess (`parent.MoveItem` SourceContainer TargetContainer SourceIdx TargetIdx InData MoveCount))
  (return _bismovesuccess))

(fn `OnContextClick`
  (params (InSlotIdx :type Integer) (InContextAction :type "/Game/GameSrc/Blueprint/Widget/HUD/Inventory/ButtenContext/EContextActionType Enum" :default "NewEnumerator0") (InEquipContainer :type "/Game/GameSrc/Blueprint/Interface/BPI_ItemContain Interface") (InTransform :type "Transform Structure"))
  (switch `/Game/GameSrc/Blueprint/Widget/HUD/Inventory/ButtenContext/EContextActionType` InContextAction
    (:`NewEnumerator0`
      (`/Game/GameSrc/Blueprint/Interface/BPI_ItemInteraction.DropItem` InSlotIdx 1 InTransform))
    (:`NewEnumerator3`
      (`/Game/GameSrc/Blueprint/Interface/BPI_ItemInteraction.EquipItem` InSlotIdx InEquipContainer))))

(fn `RemoveItem`
  (params (InIdx :type Integer) (InCount :type Integer))
  (returns (bIsSuccess :type Boolean))
  (bind _bissuccess (`parent.RemoveItem` InIdx InCount))
  (if _bissuccess
    (bind _outdata (`/Game/GameSrc/Blueprint/Interface/BPI_ItemContain.GetItem` InIdx))
    (bind _outweight (`self.GetItemWeight` _outdata InCount))
    (set `self.CurrentWeight` (- (`self.CurrentWeight`) _outweight))
    (`self.OnInventoryChange` InIdx)
    (return true)
    (else
      (return false))))