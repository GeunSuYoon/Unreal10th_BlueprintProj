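; Player character Blueprint with camera-relative movement, jump, a timeline-driven dash and independent left/right weapons fired at the cursor.
; Tick traces under the cursor to yaw the actor toward it and position an aim widget, whose creation code is currently disconnected.
; Weapons are BP_Weapon child actors swapped by class, auto-reloading when fired empty behind per-hand guard flags.
; Dispatcher calls report weapon, ammo and reload changes for the UI.
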(event `self.ReceiveBeginPlay`
  (`parent.ReceiveBeginPlay`)
  ; 양손 무기 초기화
  (`self.LeftWeaponUpdate` (`self.LeftWeaponClass`))
  (`self.RightWeaponUpdate` (`self.RightWeaponClass`))
  ; UI 초기화
  (`self.HPStatusChange`)
  (`self.OnLeftWeaponChange` (`self.LeftWeaponRef`))
  (`self.OnRightWeaponChange` (`self.RightWeaponRef`)))

(event `EnhancedInput|/Game/GameSrc/Controller/IA_SetMoveKeyInput`
  (params (ActionValue :type "Vector2D Structure") (ElapsedSeconds :type "Float (double-precision)") (TriggeredSeconds :type "Float (double-precision)") (InputAction :type "InputAction Object Reference" :default "/Game/GameSrc/Controller/IA_SetMoveKeyInput.IA_SetMoveKeyInput"))
  (bind _camera (`self.Camera`))
  (bind _camera_2 (`self.Camera`))
  (bind (_returnvalue_x _returnvalue_y _returnvalue_z) (`KismetMathLibrary.BreakVector` (+ (* ActionValue_Y (`SceneComponent.GetForwardVector` _camera_2)) (* ActionValue_X (`SceneComponent.GetRightVector` _camera_2)))))
  (bind (_returnvalue_x_2 _returnvalue_y_2 _returnvalue_z_2) (`KismetMathLibrary.BreakVector` (+ (* ActionValue_Y (`SceneComponent.GetForwardVector` _camera)) (* ActionValue_X (`SceneComponent.GetRightVector` _camera)))))
  ; 이동(WASD)
  (:`Triggered`
    (if (`NavMovementComponent.IsFalling` (`self.CharacterMovement`))
      _
      (elif (not (`self.bIsDash`))
        (bind _output_get (set `self.MoveDir` (`KismetMathLibrary.MakeVector` _returnvalue_x_2 _returnvalue_y_2 _returnvalue_z_2)))
        (`self.AddMovementInput` _output_get (`self.MoveSpeed`))
        (set `self.StoreDir` _output_get))))
  (:`Completed`
    (bind _output_get_2 (set `self.MoveDir` (`KismetMathLibrary.MakeVector` _returnvalue_x _returnvalue_y _returnvalue_z)))
    (`self.AddMovementInput` _output_get_2 (`self.MoveSpeed`))))

(event `self.ReceiveTick`
  (params (DeltaSeconds :type "Float (single-precision)"))
  (`self.MacroMouseController` DeltaSeconds))

(event `EnhancedInput|/Game/GameSrc/Controller/IA_SetDashInput`
  (params (ActionValue :type Boolean) (ElapsedSeconds :type "Float (double-precision)") (TriggeredSeconds :type "Float (double-precision)") (InputAction :type "InputAction Object Reference" :default "/Game/GameSrc/Controller/IA_SetDashInput.IA_SetDashInput"))
  ; 회피(LShift)
  (:`Triggered`
    (if (not (`NavMovementComponent.IsFalling` (`self.CharacterMovement`)))
      (set `self.bIsDash` true)
      (`Timeline|타임라인` :!via `PlayFromStart`
        (:`Update`
          (`self.AddMovementInput` (* (0.0 0.0 0.0) (stale `self.ReceiveTick` DeltaSeconds) (`self.DashStrength`) (`self.StoreDir`))))
        (:`Finished`
          (`KismetSystemLibrary.Delay` 0.2)
          (set `self.bIsDash` false))))))

(event `EnhancedInput|/Game/GameSrc/Controller/IA_SetJumpKeyInput`
  (params (ActionValue :type Boolean) (ElapsedSeconds :type "Float (double-precision)") (TriggeredSeconds :type "Float (double-precision)") (InputAction :type "InputAction Object Reference" :default "/Game/GameSrc/Controller/IA_SetJumpKeyInput.IA_SetJumpKeyInput"))
  ; 점프(Space)
  (:`Triggered`
    (if (not (`self.bIsDash`))
      (set `self.bIsJump` true)
      (`self.Jump`)
      (set `self.bIsJump` false))))

(event `EnhancedInput|/Game/GameSrc/Controller/IA_SetFireLeftInput`
  (params (ActionValue :type Boolean) (ElapsedSeconds :type "Float (double-precision)") (TriggeredSeconds :type "Float (double-precision)") (InputAction :type "InputAction Object Reference" :default "/Game/GameSrc/Controller/IA_SetFireLeftInput.IA_SetFireLeftInput"))
  (bind _leftweaponref (`self.LeftWeaponRef`))
  ; 마우스 좌클릭 혹은 우클릭으로 무기 공격
  (:`Triggered`
    (if (> (`/Game/GameSrc/Blueprint/Weapon/BP_Weapon.AmmoCurrent` _leftweaponref) 0)
      (message `/Game/GameSrc/Blueprint/Interface/BPI_Attack.Attack` _leftweaponref (`.Location` (`GameplayStatics.BreakHitResult` (`PlayerController.GetHitResultUnderCursorByChannel` (`GameplayStatics.GetPlayerController` 0) "TraceTypeQuery1" false))))
      (`self.OnLeftWeaponAmmoUpdate` (`/Game/GameSrc/Blueprint/Weapon/BP_Weapon.AmmoCurrent` _leftweaponref) (`.MagazineSize_26_3C34E584416B12C1D5AC458C1D8BF996` (break `/Game/GameSrc/Blueprint/Weapon/ST_FWeaponData` (`/Game/GameSrc/Blueprint/Weapon/BP_Weapon.WeaponData` _leftweaponref))))
      (else
        (`self.MacroLeftWeaponReload`)))))

(event `EnhancedInput|/Game/GameSrc/Controller/IA_SetFireRightInput`
  (params (ActionValue :type Boolean) (ElapsedSeconds :type "Float (double-precision)") (TriggeredSeconds :type "Float (double-precision)") (InputAction :type "InputAction Object Reference" :default "/Game/GameSrc/Controller/IA_SetFireRightInput.IA_SetFireRightInput"))
  (bind _rightweaponref (`self.RightWeaponRef`))
  ; 마우스 좌클릭 혹은 우클릭으로 무기 공격
  (:`Triggered`
    (if (> (`/Game/GameSrc/Blueprint/Weapon/BP_Weapon.AmmoCurrent` _rightweaponref) 0)
      (message `/Game/GameSrc/Blueprint/Interface/BPI_Attack.Attack` _rightweaponref (`.Location` (`GameplayStatics.BreakHitResult` (`PlayerController.GetHitResultUnderCursorByChannel` (`GameplayStatics.GetPlayerController` 0) "TraceTypeQuery1" false))))
      (`self.OnRightWeaponAmmoUpdate` (`/Game/GameSrc/Blueprint/Weapon/BP_Weapon.AmmoCurrent` _rightweaponref) (`.MagazineSize_26_3C34E584416B12C1D5AC458C1D8BF996` (break `/Game/GameSrc/Blueprint/Weapon/ST_FWeaponData` (`/Game/GameSrc/Blueprint/Weapon/BP_Weapon.WeaponData` _rightweaponref))))
      (else
        (`self.MacroRightWeaponReload`)))))

(event `EventCallLeftReloadEnd`
  (bind _leftweaponref (`self.LeftWeaponRef`))
  (`self.OnLeftWeaponAmmoUpdate` (`/Game/GameSrc/Blueprint/Weapon/BP_Weapon.AmmoCurrent` _leftweaponref) (`.MagazineSize_26_3C34E584416B12C1D5AC458C1D8BF996` (break `/Game/GameSrc/Blueprint/Weapon/ST_FWeaponData` (`/Game/GameSrc/Blueprint/Weapon/BP_Weapon.WeaponData` _leftweaponref)))))

(event `EventCallRightReloadEnd`
  (bind _rightweaponref (`self.RightWeaponRef`))
  (`self.OnRightWeaponAmmoUpdate` (`/Game/GameSrc/Blueprint/Weapon/BP_Weapon.AmmoCurrent` _rightweaponref) (`.MagazineSize_26_3C34E584416B12C1D5AC458C1D8BF996` (break `/Game/GameSrc/Blueprint/Weapon/ST_FWeaponData` (`/Game/GameSrc/Blueprint/Weapon/BP_Weapon.WeaponData` _rightweaponref)))))

(fn `LeftWeaponUpdate`
  (params (InLeftWeaponClass :type "Actor Class Reference"))
  (bind _leftweapon (`self.LeftWeapon`))
  (bind _output_get (set `self.LeftWeaponClass` InLeftWeaponClass))
  (`ChildActorComponent.SetChildActorClass` _leftweapon _output_get)
  (bind _asbp_weapon (cast `/Game/GameSrc/Blueprint/Weapon/BP_Weapon` (`ChildActorComponent.ChildActor` _leftweapon))
    (:`then`
      (bind _output_get_2 (set `self.LeftWeaponRef` _asbp_weapon))
      (`self.OnLeftWeaponChange` _output_get_2)
      (add `/Game/GameSrc/Blueprint/Weapon/BP_Weapon.OnReloadFinish` _output_get_2 (`|CreateDelegate` :!event `EventCallLeftReloadEnd`)))
    (:`CastFailed`
      (`KismetSystemLibrary.PrintString` "Error: LeftWeaponUpdateFail")))
  (return))

(fn `ResetIsLeftWeaponReload`
  (set `self.bIsLeftWeaponReload` false)
  (`self.EventCallLeftReloadEnd`))

(fn `ResetIsRightWeaponReload`
  (set `self.bIsRightWeaponReload` false)
  (`self.EventCallRightReloadEnd`))

(fn `RightWeaponUpdate`
  (params (RightWeaponClass :type "Actor Class Reference"))
  (bind _rightweapon (`self.RightWeapon`))
  (bind _output_get (set `self.RightWeaponClass` RightWeaponClass))
  (`ChildActorComponent.SetChildActorClass` _rightweapon _output_get)
  (bind _asbp_weapon (cast `/Game/GameSrc/Blueprint/Weapon/BP_Weapon` (`ChildActorComponent.ChildActor` _rightweapon))
    (:`then`
      (bind _output_get_2 (set `self.RightWeaponRef` _asbp_weapon))
      (`self.OnRightWeaponChange` _output_get_2)
      (add `/Game/GameSrc/Blueprint/Weapon/BP_Weapon.OnReloadFinish` _output_get_2 (`|CreateDelegate` :!event `EventCallRightReloadEnd`)))
    (:`CastFailed`
      (`KismetSystemLibrary.PrintString` "Error: RightWeaponUpdateFail")))
  (return))

(fn `UserConstructionScript`)

(fn `새 함수`)