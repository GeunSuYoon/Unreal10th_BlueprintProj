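; BP_NormalUnit is a unit Blueprint that carries a weapon in each hand and manages reloading separately per hand.
; On BeginPlay it sets each hand's child actor to its weapon class, caches the BP_Weapon reference and assigns its hand.
; WeaponReload skips a hand already flagged as reloading; otherwise it sets the flag, starts a ReloadTime timer and calls the weapon's Reload immediately, without waiting for the timer.
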(event `self.ReceiveBeginPlay`
  (`parent.ReceiveBeginPlay`)
  ; 양손 무기 초기화
  (`self.LeftWeaponUpdate` (`self.LeftWeaponClass`))
  (`self.RightWeaponUpdate` (`self.RightWeaponClass`)))

(event `self.ReceiveTick`
  (params (DeltaSeconds :type "Float (single-precision)")))

(event `/Game/GameSrc/Blueprint/Interface/BPI_Combat.FireMotion`
  (params (InClass :type "/Game/GameSrc/Blueprint/Item/Weapon/WeaponData/EWeaponClass Enum" :default "NewEnumerator0") (InHand :type "/Game/GameSrc/Blueprint/Item/Weapon/WeaponData/EWeaponHand Enum" :default "NewEnumerator0")))

(fn `LeftWeaponUpdate`
  (params (InLeftWeaponClass :type "Actor Class Reference"))
  (bind _leftweapon (`self.LeftWeapon`))
  (bind _output_get (set `self.LeftWeaponClass` InLeftWeaponClass))
  (`ChildActorComponent.SetChildActorClass` _leftweapon _output_get)
  (bind _asbp_weapon (cast `/Game/GameSrc/Blueprint/Item/Weapon/BP_Weapon` (`ChildActorComponent.ChildActor` _leftweapon))
    (:`then`
      (bind _output_get_2 (set `self.LeftWeaponRef` _asbp_weapon))
      (`/Game/GameSrc/Blueprint/Item/Weapon/BP_Weapon.SetHand` _output_get_2 "NewEnumerator1"))
    (:`CastFailed`
      (`KismetSystemLibrary.PrintString` "Error: LeftWeaponUpdateFail")))
  (return))

(fn `ResetIsLeftWeaponReload`
  (set `self.bIsLeftWeaponReload` false))

(fn `ResetIsRightWeaponReload`
  (set `self.bIsRightWeaponReload` false))

(fn `RightWeaponUpdate`
  (params (RightWeaponClass :type "Actor Class Reference"))
  (bind _rightweapon (`self.RightWeapon`))
  (bind _output_get (set `self.RightWeaponClass` RightWeaponClass))
  (`ChildActorComponent.SetChildActorClass` _rightweapon _output_get)
  (bind _asbp_weapon (cast `/Game/GameSrc/Blueprint/Item/Weapon/BP_Weapon` (`ChildActorComponent.ChildActor` _rightweapon))
    (:`then`
      (set `self.RightWeaponRef` _asbp_weapon)
      (`/Game/GameSrc/Blueprint/Item/Weapon/BP_Weapon.SetHand` _asbp_weapon "NewEnumerator2"))
    (:`CastFailed`
      (`KismetSystemLibrary.PrintString` "Error: RightWeaponUpdateFail")))
  (return))

(fn `UserConstructionScript`)

(fn `WeaponReload`
  (params (InWeapon :type "/Game/GameSrc/Blueprint/Item/Weapon/BP_Weapon Object Reference"))
  (switch `/Game/GameSrc/Blueprint/Item/Weapon/WeaponData/EWeaponHand` (`/Game/GameSrc/Blueprint/Item/Weapon/BP_Weapon.Hand` InWeapon)
    (:`NewEnumerator1`
      (if (not (`self.bIsLeftWeaponReload`))
        (`self.WeaponReloadPrepare` InWeapon)
        (`self.WeaponReloadEnd` InWeapon)))
    (:`NewEnumerator2`
      (if (not (`self.bIsRightWeaponReload`))
        (`self.WeaponReloadPrepare` InWeapon)
        (`self.WeaponReloadEnd` InWeapon))))
  (return))

(fn `WeaponReloadEnd`
  (params (InWeapon :type "/Game/GameSrc/Blueprint/Item/Weapon/BP_Weapon Object Reference"))
  (switch `/Game/GameSrc/Blueprint/Item/Weapon/WeaponData/EWeaponHand` (`/Game/GameSrc/Blueprint/Item/Weapon/BP_Weapon.Hand` InWeapon)
    (:`NewEnumerator1`
      (`/Game/GameSrc/Blueprint/Item/Weapon/BP_Weapon.Reload` InWeapon))
    (:`NewEnumerator2`
      (`/Game/GameSrc/Blueprint/Item/Weapon/BP_Weapon.Reload` InWeapon)))
  (return))

(fn `WeaponReloadPrepare`
  (params (InWeapon :type "/Game/GameSrc/Blueprint/Item/Weapon/BP_Weapon Object Reference"))
  (bind (_weaponname _weaponcategory _weaponclass _ammotype _ammospeed _damage _firerate _reloadtime) (break `/Game/GameSrc/Blueprint/Item/Weapon/WeaponData/ST_FWeaponData` (`/Game/GameSrc/Blueprint/Item/Weapon/BP_Weapon.WeaponData` InWeapon)))
  (switch `/Game/GameSrc/Blueprint/Item/Weapon/WeaponData/EWeaponHand` (`/Game/GameSrc/Blueprint/Item/Weapon/BP_Weapon.Hand` InWeapon)
    (:`NewEnumerator1`
      (set `self.bIsLeftWeaponReload` true)
      (`KismetSystemLibrary.K2_SetTimerDelegate` (`|CreateDelegate` :!event `ResetIsLeftWeaponReload`) _reloadtime))
    (:`NewEnumerator2`
      (set `self.bIsRightWeaponReload` true)
      (`KismetSystemLibrary.K2_SetTimerDelegate` (`|CreateDelegate` :!event `ResetIsRightWeaponReload`) _reloadtime)))
  (return))