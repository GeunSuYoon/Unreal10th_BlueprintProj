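; BP_Unit is a Character-based unit Blueprint that handles HP, defense, damage, healing and death.
; On BeginPlay it caches a defense multiplier of 100/(100+Defense), sets walk speed and binds its WBP_DamageText widget to itself.
; TakeDamage applies that multiplier and broadcasts hit and HP-change events, which RestoreHP also does for HP changes.
; At zero HP, UnitDie clears IsAlive and calls ReceiveDeath, which only prints a message here.
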(event `self.ReceiveBeginPlay`
  (bind _returnvalue (`WidgetComponent.GetUserWidgetObject` (`self.DamageTextWidget`)))
  (`self.SetDefenseRate`)
  (set `CharacterMovementComponent.MaxWalkSpeed` (`self.MoveSpeed`) (`self.CharacterMovement`))
  (`/Engine/EditorBlueprintResources/StandardMacros.IsValid` _returnvalue
    (:`Is Valid`
      (bind _aswbp_damage_text (cast `/Game/GameSrc/Blueprint/Widget/WBP_DamageText` _returnvalue)
        (:`then`
          (`/Game/GameSrc/Blueprint/Widget/WBP_DamageText.BindToUnit` _aswbp_damage_text self))
        (:`CastFailed`
          (`KismetSystemLibrary.PrintString` "TextWidgetCastFail"))))))

(fn `HPStatusChange`
  (`self.OnHPChanged` (`self.HPCurrent`) (`self.HPMax`))
  (return))

(fn `ReceiveDeath`
  (`KismetSystemLibrary.PrintString` "Unit Death"))

(fn `RestoreHP`
  (params (InHeal :type "Float (double-precision)"))
  (set `self.HPCurrent` (`KismetMathLibrary.FMin` (+ InHeal (`self.HPCurrent`)) (`self.HPMax`)))
  (`self.HPStatusChange`)
  (return))

(fn `TakeDamage`
  (params (InDamage :type "Float (double-precision)"))
  (bind _returnvalue (* (`self.DefenseRate`) InDamage))
  ; 방어력 기반 받는 데미지 계산 후 체력에서 제외
  (bind _output_get (set `self.HPCurrent` (`KismetMathLibrary.FMax` (- (`self.HPCurrent`) _returnvalue))))
  (`self.OnHitByEnemy` _returnvalue)
  (`self.HPStatusChange`)
  (if (<= _output_get 0.0)
    (`self.UnitDie`))
  (return))

(fn `UnitDie`
  (set `self.bIsAlive` false)
  (`self.ReceiveDeath`)
  (return))

(fn `UserConstructionScript`)