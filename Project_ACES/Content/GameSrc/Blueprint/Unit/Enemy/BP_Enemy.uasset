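; Enemy unit Blueprint that fights the player with two child-actor weapons and shows a bound HP bar.
; Looping timers are set up at BeginPlay, and Tick turns its yaw toward the player.
; Squared-distance checks with randomized thresholds choose between chasing a detected player and shifting diagonally backward left or right.
; Within the left weapon's range it fires both weapons, each reloading independently when empty.
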(event `self.ReceiveBeginPlay`
  (bind _leftweapon (`self.LeftWeapon`))
  (bind _rightweapon (`self.RightWeapon`))
  (`parent.ReceiveBeginPlay`)
  (set `self.DetectSquare` (`KismetMathLibrary.Square` (`self.DetectRange`)))
  ; 양손 무기 초기화
  (`ChildActorComponent.SetChildActorClass` _leftweapon (`self.LeftWeaponClass`))
  (bind _asbp_weapon (cast `/Game/GameSrc/Blueprint/Weapon/BP_Weapon` (`ChildActorComponent.ChildActor` _leftweapon)))
  (bind _output_get (set `self.LeftWeaponRef` _asbp_weapon))
  (`ChildActorComponent.SetChildActorClass` _rightweapon (`self.RightWeaponClass`))
  (bind _asbp_weapon_2 (cast `/Game/GameSrc/Blueprint/Weapon/BP_Weapon` (`ChildActorComponent.ChildActor` _rightweapon)))
  (set `self.RightWeaponRef` _asbp_weapon_2)
  (bind (_weaponname _weaponcategory _weaponclass _ammotype _ammospeed _damage _firerate _reloadtime _magazinesize _range) (break `/Game/GameSrc/Blueprint/Weapon/ST_FWeaponData` (`/Game/GameSrc/Blueprint/Weapon/BP_Weapon.WeaponData` _output_get)))
  (bind _output_get_2 (set `self.PreferredDist` _range))
  (set `self.PreferredDistSquare` (* _output_get_2 _range))
  (`KismetSystemLibrary.K2_SetTimerDelegate` (`|CreateDelegate` :!event `TryAttack`) 0.2 true)
  (`KismetSystemLibrary.K2_SetTimerDelegate` (`|CreateDelegate` :!event `TryMovement`) 1.0 true)
  ; HP바 바인딩
  (bind _aswbp_hpbar (cast `/Game/GameSrc/Blueprint/Widget/WBP_HPBar` (`WidgetComponent.GetUserWidgetObject` (`self.HPBarWidget`))))
  (`/Game/GameSrc/Blueprint/Widget/WBP_HPBar.BindToUnit` _aswbp_hpbar self)
  (`self.OnHPChanged` (`self.HPCurrent`) (`self.HPMax`)))

(event `TryAttack`
  (bind _returnvalue (`self.K2_GetActorLocation` (`GameplayStatics.GetPlayerCharacter` 0)))
  (if (`self.bMacroIsPreferredChecker` (`KismetMathLibrary.Vector_DistanceSquared` (`self.K2_GetActorLocation`) _returnvalue))
    (`self.MacroAttackPlayer` _returnvalue)))

(event `TryMovement`
  (bind _returnvalue (`GameplayStatics.GetPlayerCharacter` 0))
  (bind _returnvalue_2 (`self.K2_GetActorLocation`))
  (bind _returnvalue_3 (`self.K2_GetActorLocation` _returnvalue))
  (bind _returnvalue_4 (`KismetMathLibrary.Vector_DistanceSquared` _returnvalue_2 _returnvalue_3))
  (if (`self.bMacroIsDetectedChecker` _returnvalue_4)
    (if (`self.bMacroIsCloseChecker` _returnvalue_4)
      (`|AIMoveTo` (`self.GetController`) null (0.0 0.0 0.0) _returnvalue 5.0 true)
      (else
        (`self.MacroShifter` _returnvalue_2 (`KismetMathLibrary.FindLookAtRotation` _returnvalue_2 _returnvalue_3))))))

(event `self.ReceiveTick`
  (params (DeltaSeconds :type "Float (single-precision)"))
  (`self.MacroEnemyRot` (`KismetMathLibrary.FindLookAtRotation` (`self.K2_GetActorLocation`) (`self.K2_GetActorLocation` (`GameplayStatics.GetPlayerCharacter` 0))) DeltaSeconds))

(fn `LeftReload`
  (bind _leftweaponref (`self.LeftWeaponRef`))
  (if (not (`self.bIsLeftReload`))
    (set `self.bIsLeftReload` true)
    (`KismetSystemLibrary.K2_SetTimerDelegate` (`|CreateDelegate` :!event `LeftReloadReset`) (`.ReloadTime_23_3F687E204BDC5D1B060F668CA3030DFE` (break `/Game/GameSrc/Blueprint/Weapon/ST_FWeaponData` (`/Game/GameSrc/Blueprint/Weapon/BP_Weapon.WeaponData` _leftweaponref))))
    (`/Game/GameSrc/Blueprint/Weapon/BP_Weapon.Reload` _leftweaponref))
  (return))

(fn `LeftReloadReset`
  (set `self.bIsLeftReload` false))

(fn `ReceiveDeath`
  (`self.K2_DestroyActor`)
  (`self.K2_DestroyActor`)
  (`KismetSystemLibrary.PrintString` "Enemy Death")
  (`self.K2_DestroyActor`))

(fn `RightReload`
  (bind _rightweaponref (`self.RightWeaponRef`))
  (if (not (`self.bIsRightReload`))
    (set `self.bIsRightReload` true)
    (`KismetSystemLibrary.K2_SetTimerDelegate` (`|CreateDelegate` :!event `RightReloadReset`) (`.ReloadTime_23_3F687E204BDC5D1B060F668CA3030DFE` (break `/Game/GameSrc/Blueprint/Weapon/ST_FWeaponData` (`/Game/GameSrc/Blueprint/Weapon/BP_Weapon.WeaponData` _rightweaponref))))
    (`/Game/GameSrc/Blueprint/Weapon/BP_Weapon.Reload` _rightweaponref))
  (return))

(fn `RightReloadReset`
  (set `self.bIsRightReload` false))

(fn `UserConstructionScript`)