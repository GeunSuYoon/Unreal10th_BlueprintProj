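; BP_PickupItem is a world item pickup that players can collect into their inventory.
; On BeginPlay it fetches item data from the GameInstance by RawName, falling back to its stored instance ID, and sets the mesh.
; For RawName items lacking valid instance data, it builds type-specific default state.
; Overlap with BPI_IPlayer actors toggles the widget; PickUp passes instance and count to the player's inventory, destroying itself on success.
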(event `self.ReceiveBeginPlay`
  (bind (_outdata _outisvaliddata) (message `/Game/GameSrc/Blueprint/Interface/BPI_DataTableHandle.GetItemData` (`GameplayStatics.GetGameInstance`) (`self.RawName`)))
  (if _outisvaliddata
    (bind _output_get (set `self.ItemData` _outdata))
    (`StaticMeshComponent.SetStaticMesh` (`self.StaticMesh`) (`.Mesh_30_DBB0559B4EE1DAB84D170CB9DD6D3F3E` (break `/Game/GameSrc/Blueprint/Item/ST_FItemData` _output_get)))
    (`SceneComponent.SetVisibility` (`self.Widget`) false false)
    (`self.InitItemInstanceData`)
    (else
      (bind _outdata_2 (message `/Game/GameSrc/Blueprint/Interface/BPI_DataTableHandle.GetItemData` (`GameplayStatics.GetGameInstance`) (`.ItemID_2_8E977A954A28F24960B39DB752D5296B` (break `/Game/GameSrc/Blueprint/ItemContain/Structure/ST_FItemInstance` (`self.ItemInstanceData`)))))
      (bind _output_get_2 (set `self.ItemData` _outdata_2))
      (`StaticMeshComponent.SetStaticMesh` (`self.StaticMesh`) (`.Mesh_30_DBB0559B4EE1DAB84D170CB9DD6D3F3E` (break `/Game/GameSrc/Blueprint/Item/ST_FItemData` _output_get_2)))
      (`SceneComponent.SetVisibility` (`self.Widget`) false false))))

(event `self.ReceiveActorBeginOverlap`
  (params (OtherActor :type "Actor Object Reference"))
  (if (`KismetSystemLibrary.DoesImplementInterface` OtherActor "/Game/GameSrc/Blueprint/Interface/BPI_IPlayer.BPI_IPlayer_C")
    (`SceneComponent.SetVisibility` (`self.Widget`) true false)))

(event `self.ReceiveActorEndOverlap`
  (params (OtherActor :type "Actor Object Reference"))
  (if (`KismetSystemLibrary.DoesImplementInterface` OtherActor "/Game/GameSrc/Blueprint/Interface/BPI_IPlayer.BPI_IPlayer_C")
    (`SceneComponent.SetVisibility` (`self.Widget`) false false)))

(event `/Game/GameSrc/Blueprint/Interface/BPI_Interact.PickUp`
  (params (InPlayer :type "/Game/GameSrc/Blueprint/Unit/BP_Player Object Reference"))
  (bind _boutissuccess (message `/Game/GameSrc/Blueprint/Interface/BPI_ItemContain.AddItem` (`ChildActorComponent.ChildActor` (`/Game/GameSrc/Blueprint/Unit/BP_Player.Inventory` InPlayer)) (`self.ItemInstanceData`) (`self.Count`)))
  (if _boutissuccess
    (`self.K2_DestroyActor`)))

(fn `InitItemInstanceData`
  (bind (_id _name _rarity _itemtype) (break `/Game/GameSrc/Blueprint/Item/ST_FItemData` (`self.ItemData`)))
  (bind (_outdata _outisvaliddata) (message `/Game/GameSrc/Blueprint/Interface/BPI_DataTableHandle.GetItemData` (`GameplayStatics.GetGameInstance`) (`.ItemID_2_8E977A954A28F24960B39DB752D5296B` (break `/Game/GameSrc/Blueprint/ItemContain/Structure/ST_FItemInstance` (`self.ItemInstanceData`)))))
  (if (not _outisvaliddata)
    (switch `/Game/GameSrc/Blueprint/Item/EItemType` _itemtype
      (:`NewEnumerator0`
        (bind (_outdata_2 _outisvaliddata_2) (message `/Game/GameSrc/Blueprint/Interface/BPI_DataTableHandle.GetUnitPartsData` (`GameplayStatics.GetGameInstance`) _id))
        (if _outisvaliddata_2
          (set `self.ItemInstanceData` (make `/Game/GameSrc/Blueprint/ItemContain/Structure/ST_FItemInstance` _id _itemtype (struct) (make `/Game/GameSrc/Blueprint/ItemContain/Structure/ST_FUnitPartsState` (`.PartsType_9_543EAEA0432F59176BB0AEA58949A9F3` (break `/Game/GameSrc/Blueprint/Item/UnitParts/ST_UnitPartsData` _outdata_2)) 100.0)))))
      (:`NewEnumerator1`
        (set `self.ItemInstanceData` (make `/Game/GameSrc/Blueprint/ItemContain/Structure/ST_FItemInstance` _id _itemtype (make `/Game/GameSrc/Blueprint/ItemContain/Structure/ST_FWeaponState` 100.0 0 null null null))))
      (:`NewEnumerator2`
        (set `self.ItemInstanceData` (make `/Game/GameSrc/Blueprint/ItemContain/Structure/ST_FItemInstance` _id _itemtype) :!label _label))
      (:`NewEnumerator3`
        (goto _label))
      (:`NewEnumerator4`
        (goto _label)))))

(fn `UserConstructionScript`)