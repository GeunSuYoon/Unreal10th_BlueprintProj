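; BP_Ammo is a projectile actor that damages units and serves as the default despawn logic for bullets, including guided and grenade variants.
; BeginPlay sets its mesh from item data by ID, ignores GameTraceChannel1 and caches squared range.
; Tick destroys it once it exceeds range from StartPos or nearly stops.
; Hits ignore the instigator and owner, damage any BP_Unit, then destroy the projectile.
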(event `self.ReceiveBeginPlay`
  (`PrimitiveComponent.SetCollisionResponseToChannel` (`self.BulletCollision`) "ECC_GameTraceChannel1" "ECR_Ignore")
  (bind _outdata (message `/Game/GameSrc/Blueprint/Interface/BPI_GIHandle.GetItemData` (`GameplayStatics.GetGameInstance`) (`self.ID`)))
  (`StaticMeshComponent.SetStaticMesh` (`self.StaticMesh`) (`.Mesh_30_DBB0559B4EE1DAB84D170CB9DD6D3F3E` (break `/Game/GameSrc/Blueprint/Item/ST_FItemData` _outdata)))
  (set `self.RangeSquare` (* (`self.Range`) (`self.Range`))))

(event `self.ReceiveTick`
  (params (DeltaSeconds :type "Float (single-precision)"))
  ; 기본적인 총알 없어짐 로직. 일반 총알 외 유도탄, 류탄 등도 있으므로 해당 로직을 기본으로 한다.
  (if (>= (`KismetMathLibrary.Vector_DistanceSquared` (`self.K2_GetActorLocation`) (`self.StartPos`)) (`self.RangeSquare`))
    (`self.K2_DestroyActor` :!label _label)
    (elif (< (`KismetMathLibrary.VSizeSquared` (`MovementComponent.Velocity` (`self.ProjectileMovement`))) 100.0)
      (goto _label))))

(event `self.BulletCollision.OnComponentHit`
  (params (HitComponent :type "PrimitiveComponent Object Reference") (OtherActor :type "Actor Object Reference") (OtherComp :type "PrimitiveComponent Object Reference") (NormalImpulse :type "Vector Structure") (Hit :type "HitResult Structure (by ref)"))
  (`self.HitSomeObj` OtherActor))

(fn `HitSomeObj`
  (params (InObject :type "Object Object Reference"))
  ; 충돌한 오브젝트가 총 주인 혹은 총인지 판별
  (if (== InObject (`self.GetInstigator`))
    _
    (elif (not (== InObject (`self.GetOwner`)))
      ; 충돌한 오브젝트가 bp_unit인지 판별
      (bind _asbp_unit (cast `/Game/GameSrc/Blueprint/Unit/BP_Unit` InObject)
        (:`then`
          ; 데미지 주기
          (`/Game/GameSrc/Blueprint/Unit/BP_Unit.TakeDamage` _asbp_unit (`self.Damage`)))
        (:`CastFailed`
          _))
      (`self.K2_DestroyActor`))))

(fn `UserConstructionScript`)