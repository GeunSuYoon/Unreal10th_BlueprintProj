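; Ranged weapon Blueprint that fires projectiles from its muzzle and handles magazine reloading.
; Attack checks reload, ammo and cooldown state, plays a left- or right-hand pistol montage, then spawns a bullet aimed at the target flattened to muzzle height.
; WeaponData supplies the bullet's stats and the fire-rate and reload timers.
; Reload stores the incoming ammo amount, which RefillMagazine adds to the current count.
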(event `self.ReceiveBeginPlay`
  (`parent.ReceiveBeginPlay`))

(fn `Attack`
  (params (InTargetPos :type "Vector Structure"))
  (bind _isattack (`self.IsAttack`))
  (bind (_weaponcategory _weaponclass _weaponclassenum _ammotype _ammospeed _damage _firerate _reloadtime _magazinesize _range) (break `/Game/GameSrc/Blueprint/Item/Weapon/WeaponData/ST_FWeaponData` (`self.WeaponData`)))
  (bind (_returnvalue_location _returnvalue_rotation _returnvalue_scale) (`KismetMathLibrary.BreakTransform` (`SceneComponent.K2_GetComponentToWorld` (`self.MuzzlePoint`))))
  (bind _returnvalue (`SkeletalMeshComponent.GetAnimInstance` (`Character.Mesh` (`self.OwnUnit`))))
  (if (`self.bIsReload`)
    _
    (elif (> (`self.AmmoCurrent`) 0)
      (if _isattack
        (set `self.IsAttack` (not _isattack))
        (set `self.AmmoCurrent` (- (`self.AmmoCurrent`) 1))
        (switch `/Game/GameSrc/Blueprint/Item/Weapon/WeaponData/EWeaponHand` (`self.Hand`)
          (:`NewEnumerator1`
            (`AnimInstance.Montage_Play` _returnvalue "/Game/GameSrc/Animation/Battle/MT_Pistol_Left_Idle.MT_Pistol_Left_Idle" 10.0 "MontageLength" 0.0 false))
          (:`NewEnumerator2`
            (`AnimInstance.Montage_Play` _returnvalue "/Game/GameSrc/Animation/Battle/MT_Pistol_Right_Idle.MT_Pistol_Right_Idle" 10.0 "MontageLength" 0.0 false)))
        ; Bullet Object 스폰 후 라이프 타임 및 속력 설정
        (bind _returnvalue_2 (`|SpawnActorFromClass` (`self.BulletClass`) (`KismetMathLibrary.MakeTransform` _returnvalue_location (`KismetMathLibrary.FindLookAtRotation` _returnvalue_location (`KismetMathLibrary.MakeVector` (.x InTargetPos) (.y InTargetPos) (.z _returnvalue_location))) _returnvalue_scale) "AdjustIfPossibleButAlwaysSpawn" "MultiplyWithRoot" self _damage InTargetPos _range (`.ID_2_5A92961E4BB3AF77B3715B9E7F110A1D` (break `/Game/GameSrc/Blueprint/Item/Ammo/ST_FAmmoData` _ammotype)) (`self.GetInstigator`)))
        (`ProjectileMovementComponent.SetVelocityInLocalSpace` (`/Game/GameSrc/Blueprint/Item/Ammo/BP_Ammo.ProjectileMovement` _returnvalue_2) (* (1.0 0.0 0.0) _ammospeed))
        ; Attack Rate초 이후 IsAttack true
        (`KismetSystemLibrary.K2_SetTimerDelegate` (`|CreateDelegate` :!event `ResetIsAttack`) _firerate)
        (return)))))

(fn `GetDamage`)

(fn `RefillMagazine`
  (bind _reloadammoquanity (`self.ReloadAmmoQuanity`))
  (set `self.AmmoCurrent` (+ (`self.AmmoCurrent`) _reloadammoquanity))
  (set `self.bIsReload` false)
  (`parent.Reload` _reloadammoquanity)
  (return))

(fn `Reload`
  (params (InAmmo :type Integer))
  (if (!= InAmmo 0)
    (set `self.ReloadAmmoQuanity` InAmmo)
    (set `self.bIsReload` true)
    (`KismetSystemLibrary.K2_SetTimerDelegate` (`|CreateDelegate` :!event `RefillMagazine`) (`.ReloadTime_23_3F687E204BDC5D1B060F668CA3030DFE` (break `/Game/GameSrc/Blueprint/Item/Weapon/WeaponData/ST_FWeaponData` (`self.WeaponData`))))
    (`parent.Reload` 0)
    (return)))

(fn `UserConstructionScript`)