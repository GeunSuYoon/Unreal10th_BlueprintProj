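; BP_Weapon is a weapon item actor that holds weapon data, ammo, durability and hand state.
; On BeginPlay it looks up WeaponData through the GameInstance by item ID, fills the magazine and takes a parent Character as Instigator and owning unit.
; InitInstanceData restores item data, durability and current ammo from saved instance data.
; Reload only signals completion, ResetIsAttack re-enables the attack flag, and GetUnitPartsData is an empty stub.
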(event `self.ReceiveBeginPlay`
  (bind _returnvalue (`self.GetParentActor` self))
  (`parent.ReceiveBeginPlay`)
  (bind (_outdata _outisvaliddata) (message `/Game/GameSrc/Blueprint/Interface/BPI_DataTableHandle.GetWeaponData` (`GameplayStatics.GetGameInstance`) (`.ID_40_FDD410C84A0886C929E0B3B12901A126` (break `/Game/GameSrc/Blueprint/Item/ST_FItemData` (`self.ItemData`)))))
  (if _outisvaliddata
    (set `self.WeaponData` _outdata)
    (set `self.AmmoCurrent` (`.MagazineSize_26_3C34E584416B12C1D5AC458C1D8BF996` (break `/Game/GameSrc/Blueprint/Item/Weapon/WeaponData/ST_FWeaponData` (`self.WeaponData`))))
    (`/Engine/EditorBlueprintResources/StandardMacros.IsValid` _returnvalue
      (:`Is Valid`
        (bind `_as캐릭터` (cast `Character` _returnvalue))
        (set `self.Instigator` `_as캐릭터`)
        (set `self.OwnUnit` `_as캐릭터`)))))

(fn `GetUnitPartsData`
  (returns (OutUnitPartsData :type "/Game/GameSrc/Blueprint/Item/UnitParts/ST_UnitPartsData Structure"))
  (return))

(fn `GetWeaponData`
  (returns (OutWeaponData :type "/Game/GameSrc/Blueprint/Item/Weapon/WeaponData/ST_FWeaponData Structure"))
  (return (`self.WeaponData`)))

(fn `InitInstanceData`
  (params (InData :type "/Game/GameSrc/Blueprint/ItemContain/Structure/ST_FItemInstance Structure"))
  (bind (_itemid _itemtype _weaponstate) (break `/Game/GameSrc/Blueprint/ItemContain/Structure/ST_FItemInstance` InData))
  (bind _returnvalue (`GameplayStatics.GetGameInstance`))
  (bind (_durability _currentammo) (break `/Game/GameSrc/Blueprint/ItemContain/Structure/ST_FWeaponState` _weaponstate))
  (bind _outdata (message `/Game/GameSrc/Blueprint/Interface/BPI_DataTableHandle.GetItemData` _returnvalue _itemid))
  (set `self.ItemData` _outdata)
  (bind _outdata_2 (message `/Game/GameSrc/Blueprint/Interface/BPI_DataTableHandle.GetWeaponData` _returnvalue _itemid))
  (set `self.WeaponData` _outdata_2)
  (set `self.Durability` _durability)
  (set `self.AmmoCurrent` _currentammo))

(fn `Reload`
  (`self.OnReloadFinish`)
  (return))

(fn `ResetIsAttack`
  (set `self.IsAttack` true)
  (return))

(fn `SetHand`
  (params (Hand :type "/Game/GameSrc/Blueprint/Item/Weapon/WeaponData/EWeaponHand Enum" :default "NewEnumerator0"))
  (set `self.Hand` Hand))

(fn `UserConstructionScript`)