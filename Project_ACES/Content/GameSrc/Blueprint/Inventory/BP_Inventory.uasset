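; BP_Inventory is an inventory Blueprint that stores items in an array of STFInventorySlot structs.
; AddItem increments the slot with a matching item ID, otherwise fills the first zero-quantity slot, and returns false when neither exists.
; GetItem returns a "None" item for invalid indices, while RemoveItem deletes the whole array element, shifting later indices.
; BeginPlay's MaxSlotCount loop is empty, as the node that adds empty slots is disconnected.
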(event `self.ReceiveBeginPlay`
  (for _ (range (`self.MaxSlotCount`))
    _))

(event `/Game/GameSrc/Blueprint/Interface/BPI_ItemContainer.RemoveItem`
  (params (InIdx :type Integer))
  (bind _items (`self.Items`))
  (if (`KismetArrayLibrary.Array_IsValidIndex` _items InIdx)
    (`KismetArrayLibrary.Array_Remove` _items InIdx)))

(fn `AddItem`
  (params (InData :type "/Game/GameSrc/Blueprint/Item/ST_FItemData Structure"))
  (returns (bOutIsSuccess :type Boolean))
  (bind _outidx (`self.FindItemIdx` InData))
  (if (!= _outidx -1)
    (`/Engine/EditorBlueprintResources/StandardMacros.IncrementInt` (`.Quantity_10_B3ECC0C94CC79C082E5E27B4736CC1B3` (break `/Game/GameSrc/Blueprint/Inventory/ST_FInventorySlot` (`|GetArrayItem` (`self.Items`) _outidx)))
      (:`  `
        _))
    (else
      (bind _array_index (`self.FindEmptySlot`))
      (if (!= _array_index -1)
        (`KismetArrayLibrary.Array_Set` (`self.Items`) _array_index (make `/Game/GameSrc/Blueprint/Inventory/ST_FInventorySlot` InData 1))
        (else
          (return false)))))
  (return true))

(fn `FindEmptySlot`
  (returns (`Array Index` :type Integer))
  (for (_array_element _array_index) (`self.Items`)
    (if (== (`.Quantity_10_B3ECC0C94CC79C082E5E27B4736CC1B3` (break `/Game/GameSrc/Blueprint/Inventory/ST_FInventorySlot` _array_element)) 0)
      (return _array_index)))
  (return -1))

(fn `FindItemIdx`
  (params (InData :type "/Game/GameSrc/Blueprint/Item/ST_FItemData Structure"))
  (returns (OutIdx :type Integer))
  (for (_array_element _array_index) (`self.Items`)
    (if (== (`.ID_25_FDD410C84A0886C929E0B3B12901A126` (break `/Game/GameSrc/Blueprint/Item/ST_FItemData` InData)) (`.ID_25_FDD410C84A0886C929E0B3B12901A126` (break `/Game/GameSrc/Blueprint/Item/ST_FItemData` (`.Data_11_404723F4452CFF2DB1C01F98B3B04221` (break `/Game/GameSrc/Blueprint/Inventory/ST_FInventorySlot` _array_element)))))
      (return _array_index)))
  (return -1))

(fn `GetItem`
  (params (InIdx :type Integer))
  (returns (OutData :type "/Game/GameSrc/Blueprint/Item/ST_FItemData Structure"))
  (bind _items (`self.Items`))
  (if (`KismetArrayLibrary.Array_IsValidIndex` _items InIdx)
    (return (`.Data_11_404723F4452CFF2DB1C01F98B3B04221` (break `/Game/GameSrc/Blueprint/Inventory/ST_FInventorySlot` (`|GetArrayItem` _items InIdx))))
    (else
      (return (make `/Game/GameSrc/Blueprint/Item/ST_FItemData` 0 "None" "NewEnumerator6" 0.0 0.0 0.0 null "NewEnumerator4")))))

(fn `UserConstructionScript`)