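; BP_Weapon is a weapon actor that holds ammo, attack, hand and owner state.
; On BeginPlay it fills current ammo from WeaponData's magazine size and, if its parent actor is a Character, caches that as Instigator and OwnUnit.
; Reload only fires OnReloadFinish without changing ammo, ResetIsAttack sets IsAttack to true, and SetHand stores the given hand.
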(event `self.ReceiveBeginPlay`
  (bind _returnvalue (`self.GetParentActor` self))
  (set `self.AmmoCurrent` (`.MagazineSize_26_3C34E584416B12C1D5AC458C1D8BF996` (break `/Game/GameSrc/Blueprint/Weapon/WeaponData/ST_FWeaponData` (`self.WeaponData`))))
  (`/Engine/EditorBlueprintResources/StandardMacros.IsValid` _returnvalue
    (:`Is Valid`
      (bind `_as캐릭터` (cast `Character` _returnvalue))
      (set `self.Instigator` `_as캐릭터`)
      (set `self.OwnUnit` `_as캐릭터`))))

(fn `Reload`
  (`self.OnReloadFinish`)
  (return))

(fn `ResetIsAttack`
  (set `self.IsAttack` true)
  (return))

(fn `SetHand`
  (params (Hand :type "/Game/GameSrc/Blueprint/Weapon/WeaponData/EWeaponHand Enum" :default "NewEnumerator0"))
  (set `self.Hand` Hand))

(fn `UserConstructionScript`)