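; BP_RangedWeapon is a ranged weapon Blueprint that fires projectiles toward a target position, with limited magazine ammo.
; Attack checks ammo and the IsAttack gate, then spawns a bullet at the muzzle, flattening aim to muzzle height.
; WeaponData supplies bullet stats, fire-rate and reload timers, and magazine size for RefillMagazine.
; Reload clears IsReload immediately after starting its timer, without waiting for it to finish.
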(event `self.ReceiveBeginPlay`
  (`parent.ReceiveBeginPlay`))

(fn `Attack`
  (params (InTargetPos :type "Vector Structure"))
  (bind _isattack (`self.IsAttack`))
  (bind (_weaponname _weaponcategory _weaponclass _ammotype _ammospeed _damage _firerate _reloadtime _magazinesize _range) (break `/Game/GameSrc/Blueprint/Weapon/ST_FWeaponData` (`self.WeaponData`)))
  (bind (_returnvalue_location _returnvalue_rotation _returnvalue_scale) (`KismetMathLibrary.BreakTransform` (`SceneComponent.K2_GetComponentToWorld` (`self.MuzzlePoint`))))
  (if (> (`self.AmmoCurrent`) 0)
    (if _isattack
      (set `self.IsAttack` (not _isattack))
      (set `self.AmmoCurrent` (- (`self.AmmoCurrent`) 1))
      ; Bullet Object 스폰 후 라이프 타임 및 속력 설정
      (bind _returnvalue (`|SpawnActorFromClass` (`self.BulletClass`) (`KismetMathLibrary.MakeTransform` _returnvalue_location (`KismetMathLibrary.FindLookAtRotation` _returnvalue_location (`KismetMathLibrary.MakeVector` (.x InTargetPos) (.y InTargetPos) (.z _returnvalue_location))) _returnvalue_scale) "Undefined" "MultiplyWithRoot" self _damage InTargetPos _range (`self.GetInstigator`)))
      (`ProjectileMovementComponent.SetVelocityInLocalSpace` (`/Game/GameSrc/Blueprint/Ammo/BP_Ammo.ProjectileMovement` _returnvalue) (* (1.0 0.0 0.0) _ammospeed))
      ; Attack Rate초 이후 IsAttack true
      (`KismetSystemLibrary.K2_SetTimerDelegate` (`|CreateDelegate` :!event `ResetIsAttack`) _firerate)
      (return))))

(fn `RefillMagazine`
  (set `self.AmmoCurrent` (`.MagazineSize_26_3C34E584416B12C1D5AC458C1D8BF996` (break `/Game/GameSrc/Blueprint/Weapon/ST_FWeaponData` (`self.WeaponData`))))
  (`parent.Reload`)
  (return))

(fn `Reload`
  (set `self.bIsReload` true)
  (`KismetSystemLibrary.K2_SetTimerDelegate` (`|CreateDelegate` :!event `RefillMagazine`) (`.ReloadTime_23_3F687E204BDC5D1B060F668CA3030DFE` (break `/Game/GameSrc/Blueprint/Weapon/ST_FWeaponData` (`self.WeaponData`))))
  (set `self.bIsReload` false)
  (return))

(fn `UserConstructionScript`)