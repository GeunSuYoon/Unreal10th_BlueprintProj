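; Player character Blueprint for mouse-aimed movement with WASD, jump and dash, driven by Enhanced Input.
; WASD moves relative to the camera and stores the last direction, which a timeline-driven dash follows while grounded, blocking move and jump until shortly after it ends.
; Each tick, a macro traces under the cursor, positions the aim widget at the projected hit point and turns the actor toward it on yaw only.
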(event `self.ReceiveBeginPlay`
  ; IMC 설정
  (`EnhancedInputSubsystemInterface.AddMappingContext` (subsystem `EnhancedInputLocalPlayerSubsystem`) "/Game/Input/IMC_MyIMC.IMC_MyIMC" 0 (struct))
  ; 마우스 에임 위젯 초기화
  (bind _returnvalue (`|CreateWidget` "/Game/Blueprint/WBP_Aim.WBP_Aim_C" (`GameplayStatics.GetPlayerController` 0)))
  (`UserWidget.AddToViewport` _returnvalue 0)
  (set `self.AimWidget` _returnvalue))

(event `EnhancedInput|/Game/Input/IA_SetMoveKeyInput`
  (params (ActionValue :type "Vector2D Structure") (ElapsedSeconds :type "Float (double-precision)") (TriggeredSeconds :type "Float (double-precision)") (InputAction :type "InputAction Object Reference" :default "/Game/Input/IA_SetMoveKeyInput.IA_SetMoveKeyInput"))
  (bind _camera (`self.Camera`))
  (bind (_returnvalue_x _returnvalue_y _returnvalue_z) (`KismetMathLibrary.BreakVector` (+ (* ActionValue_Y (`SceneComponent.GetForwardVector` _camera)) (* ActionValue_X (`SceneComponent.GetRightVector` _camera)))))
  ; 이동(WASD)
  (:`Triggered`
    (if (`NavMovementComponent.IsFalling` (`self.CharacterMovement`))
      _
      (elif (not (`self.bIsDash`))
        (bind _output_get (set `self.MoveDir` (`KismetMathLibrary.MakeVector` _returnvalue_x _returnvalue_y _returnvalue_z) :!label _label))
        (`self.AddMovementInput` _output_get (`self.MoveSpeed`))
        (set `self.StoreDir` _output_get))))
  (:`Completed`
    (goto _label)))

(event `self.ReceiveTick`
  (params (DeltaSeconds :type "Float (single-precision)"))
  (`self.MacroMouseController` DeltaSeconds))

(event `EnhancedInput|/Game/Input/IA_SetDashInput`
  (params (ActionValue :type Boolean) (ElapsedSeconds :type "Float (double-precision)") (TriggeredSeconds :type "Float (double-precision)") (InputAction :type "InputAction Object Reference" :default "/Game/Input/IA_SetDashInput.IA_SetDashInput"))
  ; 회피(LShift)
  (:`Started`
    (if (not (`NavMovementComponent.IsFalling` (`self.CharacterMovement`)))
      (set `self.bIsDash` true)
      (bind (_direction `_새_트랙_0`) (`Timeline|타임라인` :!via `PlayFromStart`)
        (:`Update`
          (`self.AddMovementInput` (* (stale `self.ReceiveTick` DeltaSeconds) `_새_트랙_0` (`self.DashStrength`) (`self.StoreDir`))))
        (:`Finished`
          (`KismetSystemLibrary.Delay` 0.2)
          (set `self.bIsDash` false))))))

(event `EnhancedInput|/Game/Input/IA_SetJumpKeyInput`
  (params (ActionValue :type Boolean) (ElapsedSeconds :type "Float (double-precision)") (TriggeredSeconds :type "Float (double-precision)") (InputAction :type "InputAction Object Reference" :default "/Game/Input/IA_SetJumpKeyInput.IA_SetJumpKeyInput"))
  ; 점프(Space)
  (:`Started`
    (if (not (`self.bIsDash`))
      (set `self.bIsJump` true)
      (`self.Jump`)
      (set `self.bIsJump` false))))

(fn `UserConstructionScript`)