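; Player for a mouse-aimed shooter with camera-relative movement, jump, dash and two weapons.
; BeginPlay adds the input mapping, creates the aim widget and attaches spawned weapons to left and right hand sockets.
; Each Tick, MacroMouseController traces under the cursor, moves the aim widget there and interpolates yaw toward it.
; Fire inputs attack the cursor hit point, while dash uses a timeline to push along the last move direction, blocking movement and jump.
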(event `self.ReceiveBeginPlay`
  ; IMC 설정
  (`EnhancedInputSubsystemInterface.AddMappingContext` (subsystem `EnhancedInputLocalPlayerSubsystem`) "/Game/MySrc/Input/IMC_MyIMC.IMC_MyIMC" 0 (struct))
  ; 마우스 에임 위젯 초기화
  (bind _returnvalue (`|CreateWidget` "/Game/MySrc/Blueprint/WBP_Aim.WBP_Aim_C" (`GameplayStatics.GetPlayerController` 0)))
  (`UserWidget.AddToViewport` _returnvalue 0)
  (set `self.AimWidget` _returnvalue)
  ; 양손 무기 초기화
  (bind _returnvalue_2 (`|SpawnActorFromClass` (`self.LeftWeaponClass`) (`self.GetTransform`) "Undefined" "MultiplyWithRoot" self self))
  (bind _asbp_weapon (cast `/Game/MySrc/Blueprint/Weapon/BP_Weapon` _returnvalue_2)
    (:`then`
      (bind _output_get (set `self.LeftWeapon` _asbp_weapon))
      (`self.K2_AttachToComponent` _output_get (`self.SkeletalMesh`) "LeftWeaponSocket" "SnapToTarget" "SnapToTarget" "KeepWorld" true)
      (bind _returnvalue_3 (`|SpawnActorFromClass` (`self.RightWeaponClass`) (`self.GetTransform`) "Undefined" "MultiplyWithRoot" self self))
      (bind _asbp_weapon_2 (cast `/Game/MySrc/Blueprint/Weapon/BP_Weapon` _returnvalue_3)
        (:`then`
          (bind _output_get_2 (set `self.RightWeapon` _asbp_weapon_2))
          (`self.K2_AttachToComponent` _output_get_2 (`self.SkeletalMesh`) "RightWeaponSocket" "SnapToTarget" "SnapToTarget" "KeepWorld" true))
        (:`CastFailed`
          (`KismetSystemLibrary.PrintString` "Hello"))))
    (:`CastFailed`
      (`KismetSystemLibrary.PrintString` "Hello"))))

(event `EnhancedInput|/Game/MySrc/Input/IA_SetMoveKeyInput`
  (params (ActionValue :type "Vector2D Structure") (ElapsedSeconds :type "Float (double-precision)") (TriggeredSeconds :type "Float (double-precision)") (InputAction :type "InputAction Object Reference" :default "/Game/MySrc/Input/IA_SetMoveKeyInput.IA_SetMoveKeyInput"))
  (bind _camera (`self.Camera`))
  (bind _camera_2 (`self.Camera`))
  (bind (_returnvalue_x _returnvalue_y _returnvalue_z) (`KismetMathLibrary.BreakVector` (+ (* ActionValue_Y (`SceneComponent.GetForwardVector` _camera_2)) (* ActionValue_X (`SceneComponent.GetRightVector` _camera_2)))))
  (bind (_returnvalue_x_2 _returnvalue_y_2 _returnvalue_z_2) (`KismetMathLibrary.BreakVector` (+ (* ActionValue_Y (`SceneComponent.GetForwardVector` _camera)) (* ActionValue_X (`SceneComponent.GetRightVector` _camera)))))
  ; 이동(WASD)
  (:`Triggered`
    (if (`NavMovementComponent.IsFalling` (`self.CharacterMovement`))
      _
      (elif (not (`self.bIsDash`))
        (bind _output_get (set `self.MoveDir` (`KismetMathLibrary.MakeVector` _returnvalue_x_2 _returnvalue_y_2 _returnvalue_z_2)))
        (`self.AddMovementInput` _output_get (`self.MoveSpeed`))
        (set `self.StoreDir` _output_get))))
  (:`Completed`
    (bind _output_get_2 (set `self.MoveDir` (`KismetMathLibrary.MakeVector` _returnvalue_x _returnvalue_y _returnvalue_z)))
    (`self.AddMovementInput` _output_get_2 (`self.MoveSpeed`))))

(event `self.ReceiveTick`
  (params (DeltaSeconds :type "Float (single-precision)"))
  (`self.MacroMouseController` DeltaSeconds))

(event `EnhancedInput|/Game/MySrc/Input/IA_SetDashInput`
  (params (ActionValue :type Boolean) (ElapsedSeconds :type "Float (double-precision)") (TriggeredSeconds :type "Float (double-precision)") (InputAction :type "InputAction Object Reference" :default "/Game/MySrc/Input/IA_SetDashInput.IA_SetDashInput"))
  ; 회피(LShift)
  (:`Started`
    (if (not (`NavMovementComponent.IsFalling` (`self.CharacterMovement`)))
      (set `self.bIsDash` true)
      (bind (_direction `_새_트랙_0`) (`Timeline|타임라인` :!via `PlayFromStart`)
        (:`Update`
          (`self.AddMovementInput` (* (stale `self.ReceiveTick` DeltaSeconds) `_새_트랙_0` (`self.DashStrength`) (`self.StoreDir`))))
        (:`Finished`
          (`KismetSystemLibrary.Delay` 0.2)
          (set `self.bIsDash` false))))))

(event `EnhancedInput|/Game/MySrc/Input/IA_SetJumpKeyInput`
  (params (ActionValue :type Boolean) (ElapsedSeconds :type "Float (double-precision)") (TriggeredSeconds :type "Float (double-precision)") (InputAction :type "InputAction Object Reference" :default "/Game/MySrc/Input/IA_SetJumpKeyInput.IA_SetJumpKeyInput"))
  ; 점프(Space)
  (:`Started`
    (if (not (`self.bIsDash`))
      (set `self.bIsJump` true)
      (`self.Jump`)
      (set `self.bIsJump` false))))

(event `EnhancedInput|/Game/MySrc/Input/IA_SetFireLeftInput`
  (params (ActionValue :type Boolean) (ElapsedSeconds :type "Float (double-precision)") (TriggeredSeconds :type "Float (double-precision)") (InputAction :type "InputAction Object Reference" :default "/Game/MySrc/Input/IA_SetFireLeftInput.IA_SetFireLeftInput"))
  ; 마우스 좌클릭 혹은 우클릭으로 무기 공격
  (:`Triggered`
    (`/Game/MySrc/Blueprint/Weapon/BP_Weapon.Attack` (`self.LeftWeapon`) (`.Location` (`GameplayStatics.BreakHitResult` (`PlayerController.GetHitResultUnderCursorByChannel` (`GameplayStatics.GetPlayerController` 0) "TraceTypeQuery1" false))))))

(event `EnhancedInput|/Game/MySrc/Input/IA_SetFireRightInput`
  (params (ActionValue :type Boolean) (ElapsedSeconds :type "Float (double-precision)") (TriggeredSeconds :type "Float (double-precision)") (InputAction :type "InputAction Object Reference" :default "/Game/MySrc/Input/IA_SetFireRightInput.IA_SetFireRightInput"))
  ; 마우스 좌클릭 혹은 우클릭으로 무기 공격
  (:`Triggered`
    (`/Game/MySrc/Blueprint/Weapon/BP_Weapon.Attack` (`self.RightWeapon`) (`.Location` (`GameplayStatics.BreakHitResult` (`PlayerController.GetHitResultUnderCursorByChannel` (`GameplayStatics.GetPlayerController` 0) "TraceTypeQuery1" false))))))

(fn `UserConstructionScript`)