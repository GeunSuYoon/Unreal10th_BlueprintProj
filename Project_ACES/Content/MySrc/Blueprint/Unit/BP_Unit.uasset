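; BP_Unit is a Character-based unit with health, defense, movement speed and death handling.
; BeginPlay computes a damage multiplier from Defense as 100/(100+Defense), applies MoveSpeed and binds the damage-text widget to the unit.
; TakeDamage subtracts scaled damage from HP and fires the hit and HP-changed dispatchers.
; At zero HP, UnitDie clears IsAlive and calls ReceiveDeath, which only prints a message.
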(event `self.ReceiveBeginPlay`
  (`self.SetDefenseRate`)
  (set `CharacterMovementComponent.MaxWalkSpeed` (`self.MoveSpeed`) (`self.CharacterMovement`))
  (bind _aswbp_damage_text (cast `/Game/MySrc/Blueprint/Widget/WBP_DamageText` (`WidgetComponent.GetUserWidgetObject` (`self.DamageTakeWidget`))))
  (`/Game/MySrc/Blueprint/Widget/WBP_DamageText.BindToUnit` _aswbp_damage_text self))

(fn `ReceiveDeath`
  (`KismetSystemLibrary.PrintString` "Unit Death"))

(fn `TakeDamage`
  (params (InDamage :type "Float (double-precision)"))
  (bind _returnvalue (* (`self.DefenseRate`) InDamage))
  ; 방어력 기반 받는 데미지 계산 후 체력에서 제외
  (bind _output_get (set `self.HPCurrent` (- (`self.HPCurrent`) _returnvalue)))
  (`self.OnHitByEnemy` _returnvalue)
  (`self.OnHPChanged` _output_get (`self.HPMax`))
  (if (<= _output_get 0.0)
    (`self.UnitDie`))
  (return))

(fn `UnitDie`
  (set `self.bIsAlive` false)
  (`self.ReceiveDeath`)
  (return))

(fn `UserConstructionScript`)