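; BP_Gun is a weapon Blueprint that fires BP_Bullet projectiles from its muzzle toward a target position, noted as the mouse location.
; Attack spawns the bullet at MuzzlePoint, facing the target because there is no arm-aiming animation, and launches it along local X at BulletSpeed.
; The IsAttack flag gates fire rate: Attack clears it and starts an AttackRate timer, with ResetIsAttack restoring it.
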(event `self.ReceiveBeginPlay`)

(fn `Attack`
  (params (TargetPos :type "Vector Structure"))
  (bind _isattack (`self.IsAttack`))
  (bind (_returnvalue_location _returnvalue_rotation _returnvalue_scale) (`KismetMathLibrary.BreakTransform` (`SceneComponent.K2_GetComponentToWorld` (`self.MuzzlePoint`))))
  (if _isattack
    (set `self.IsAttack` (not _isattack))
    ; Bullet Object 스폰 및 속력 설정
    (bind _returnvalue (`|SpawnActorFromClass` "/Game/MySrc/Blueprint/Bullet/BP_Bullet.BP_Bullet_C" (`KismetMathLibrary.MakeTransform` _returnvalue_location (`KismetMathLibrary.Conv_VectorToRotator` (`KismetMathLibrary.Normal` (- TargetPos _returnvalue_location))) _returnvalue_scale) "Undefined" "MultiplyWithRoot" (`self.GetOwner`) null))
    (`ProjectileMovementComponent.SetVelocityInLocalSpace` (`/Game/MySrc/Blueprint/Bullet/BP_Bullet.ProjectileMovement` _returnvalue) (* (1.0 0.0 0.0) (`self.BulletSpeed`)))
    ; Attack Rate초 이후 IsAttack true
    (`KismetSystemLibrary.K2_SetTimerDelegate` (`|CreateDelegate` :!event `ResetIsAttack`) (`self.AttackRate`))
    (return)))

(fn `ResetIsAttack`
  (set `self.IsAttack` true)
  (return))

(fn `UserConstructionScript`)