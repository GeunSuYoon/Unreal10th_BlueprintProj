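; BP_Ammo is the projectile actor that damages units, with default expiry logic meant for bullets and variants like homing rounds or grenades.
; Tick destroys it once squared distance from StartPos reaches the squared Range cached at BeginPlay.
; Overlaps call AttackUnit, which ignores instigator and owner, damages any BP_Unit, then destroys the ammo.
; Blocking hits destroy it unless the other actor's class equals UnitClass.
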(event `self.ReceiveBeginPlay`
  (set `self.RangeSquare` (* (`self.Range`) (`self.Range`))))

(event `self.ReceiveTick`
  (params (DeltaSeconds :type "Float (single-precision)"))
  ; 기본적인 총알 없어짐 로직. 일반 총알 외 유도탄, 류탄 등도 있으므로 해당 로직을 기본으로 한다.
  (if (>= (`KismetMathLibrary.Vector_DistanceSquared` (`self.K2_GetActorLocation`) (`self.StartPos`)) (`self.RangeSquare`))
    (`self.K2_DestroyActor`)))

(event `self.ReceiveActorBeginOverlap`
  (params (OtherActor :type "Actor Object Reference"))
  (`self.AttackUnit` OtherActor))

(event `self.ReceiveHit`
  (params (MyComp :type "PrimitiveComponent Object Reference") (Other :type "Actor Object Reference") (OtherComp :type "PrimitiveComponent Object Reference") (bSelfMoved :type Boolean) (HitLocation :type "Vector Structure") (HitNormal :type "Vector Structure") (NormalImpulse :type "Vector Structure") (Hit :type "HitResult Structure (by ref)"))
  (if (!= (`GameplayStatics.GetObjectClass` Other) (`self.UnitClass`))
    (`self.K2_DestroyActor`)))

(fn `UserConstructionScript`)